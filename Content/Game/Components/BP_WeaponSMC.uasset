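; BP_WeaponSMC is a weapon component that spins itself around its yaw axis.
; The AddRelativeRotBNE event adds a fixed one-degree relative yaw step per call, with no delta-time scaling; nothing in this graph calls it.
; Disconnected leftover logic holds unused experiments in random tumbling: stepping toward random target rotators and easing a random rotation rate with FInterpTo.
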(event EventAddRelativeRotBNE
  (Transformation|AddRelativeRotation (Math|Rotator|MakeRotator 0.0 0.0 1.0) false false))