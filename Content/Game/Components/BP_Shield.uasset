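; BP_Shield is a character shield component that forwards incoming damage to RemoveHP and handles the shield's lifecycle audio.
; Creation plays a start sound and attaches a stored middle sound to the component.
; Destruction and down events play different end sounds, then share cleanup that restores the character's saved walk speed, stops the middle sound and destroys the component.
; The BNE-suffixed events suggest hooks from a native parent class.
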(event EventOnCreatedBNE
  (Audio|SpawnSoundatLocation "/Game/Game/Sounds/Shield/S_Shield_Start.S_Shield_Start" (Transformation|GetWorldLocation))
  (bind _returnvalue (Audio|SpawnSoundAttached "/Game/Game/Sounds/Shield/S_Shield_Middle.S_Shield_Middle" self))
  (Variables|Default|SetSoundShieldMiddle _returnvalue))

(event EventDoDamage
  (params (Damage :type Float%20%28single-precision%29) (CallInstigator :type Player%20Controller%20Object%20Reference) (Couser :type Actor%20Object%20Reference) (DamageType :type EDamageType%20Enum :default "VE_Bullet"))
  (Class|Shield|RemoveHP Damage))

(event EventOnDestroyBNE
  (bind _soundshieldmiddle (Variables|Default|GetSoundShieldMiddle))
  (Audio|SpawnSoundatLocation "/Game/Game/Sounds/Shield/S_Shield_Destroy.S_Shield_Destroy" (Transformation|GetWorldLocation))
  (Variables|/Script/Engine.CharacterMovementComponent|SetMaxWalkSpeed (Variables|/Script/Engine.Character|GetCharacterMovement (Variables|Default|GetChar)) (Variables|Default|GetCharWalkSpeed))
  (Utilities|IsValid _soundshieldmiddle
    (:Is%20Valid
      (Audio|Components|Audio|Stop _soundshieldmiddle))
    (:Is%20Not%20Valid
      _))
  (Components|DestroyComponent))

(event EventOnDownBNE
  (bind _soundshieldmiddle (Variables|Default|GetSoundShieldMiddle))
  (Audio|SpawnSoundatLocation "/Game/Game/Sounds/Shield/S_Shield_End.S_Shield_End" (Transformation|GetWorldLocation))
  (Variables|/Script/Engine.CharacterMovementComponent|SetMaxWalkSpeed (Variables|/Script/Engine.Character|GetCharacterMovement (Variables|Default|GetChar)) (Variables|Default|GetCharWalkSpeed))
  (Utilities|IsValid _soundshieldmiddle
    (:Is%20Valid
      (Audio|Components|Audio|Stop _soundshieldmiddle))
    (:Is%20Not%20Valid
      _))
  (Components|DestroyComponent))