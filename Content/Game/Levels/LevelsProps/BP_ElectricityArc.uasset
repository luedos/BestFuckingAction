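; Destructible electric arc hazard prop with two cone electrodes, a beam between them, and colors set in the construction script.
; Character pawns entering DeathSphere join a target list that a delayed Tick loop repeatedly zaps, dropping any outside the radius.
; Each zap fires a beam from the nearer electrode, or from both for double damage when distances are nearly equal.
; Incoming damage lowers HP and destroys the actor below zero.
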(event OnComponentBeginOverlap(DeathSphere)
  (params (OverlappedComponent :type Primitive%20Component%20Object%20Reference) (OtherActor :type Actor%20Object%20Reference) (OtherComp :type Primitive%20Component%20Object%20Reference) (OtherBodyIndex :type Integer) (bFromSweep :type Boolean) (SweepResult :type Hit%20Result%20Structure%20%28by%20ref%29))
  (bind _aschar_pawn (Utilities|Casting|CastToCharPawn OtherActor))
  (Utilities|Array|AddUnique (Variables|Default|GetActorsToHit) _aschar_pawn))

(event EventDoDamage
  (params (Damage :type Float%20%28single-precision%29) (CallInstigator :type Player%20Controller%20Object%20Reference) (Couser :type Actor%20Object%20Reference) (DamageType :type EDamageType%20Enum :default "VE_Bullet"))
  (bind _output_get (Variables|Default|SetHP (- (stale _output_get) Damage)))
  (if (< _output_get 0.0)
    (Actor|DestroyActor)))

(event EventTick
  (params (DeltaSeconds :type Float%20%28single-precision%29))
  (bind _deathsphere (Variables|Default|GetDeathSphere))
  (if (!= (Utilities|Array|Length (Variables|Default|GetActorsToHit)) 0)
    (Utilities|FlowControl|Delay 1.0)
    (for _array_element (Variables|Default|GetActorsToHit)
      (Utilities|FlowControl|Delay (Math|Random|RandomFloatinRange 0.0 0.2))
      (if (> (Math|Vector|VectorLength (- (Transformation|GetWorldLocation _deathsphere) (Transformation|GetActorLocation _array_element))) (Variables|/Script/Engine.SphereComponent|GetSphereRadius _deathsphere))
        (Utilities|Array|RemoveItem (Variables|Default|GetActorsToHit) _array_element)
        (elif (Math|Float|NearlyEqual(Float) (Math|Vector|VectorLength (- (Transformation|GetActorLocation _array_element) (Transformation|GetWorldLocation (Variables|Default|GetArrow1)))) (Math|Vector|VectorLength (- (Transformation|GetActorLocation _array_element) (Transformation|GetWorldLocation (Variables|Default|GetArrow)))) 2e+02)
          (bind _returnvalue (Effects|SpawnEmitterAttached "/Game/Game/Particles/P_ElectricityShot.P_ElectricityShot" (Variables|Default|GetArrow1) "None" "0, 0,-40.000000" "0, 0, 0" "SnapToTarget"))
          (bind _returnvalue_2 (Effects|SpawnEmitterAttached "/Game/Game/Particles/P_ElectricityShot.P_ElectricityShot" (Variables|Default|GetArrow) "None" "0, 0,-40.000000" "0, 0, 0" "SnapToTarget"))
          (Class|ParticleSystemComponent|SetBeamTargetPoint _returnvalue 0 (Transformation|GetActorLocation _array_element))
          (Effects|Components|ParticleSystem|SetColorParameter _returnvalue "ParticleColor" (Variables|Default|GetArcColor))
          (Class|DamageIntarface|DoDamage(Message) _array_element (* (Variables|Default|GetArcDamage) 2.0) 0 0 "VE_Bullet")
          (else
            (if (> (Math|Vector|VectorLength (- (Transformation|GetActorLocation _array_element) (Transformation|GetWorldLocation (Variables|Default|GetArrow1)))) (Math|Vector|VectorLength (- (Transformation|GetActorLocation _array_element) (Transformation|GetWorldLocation (Variables|Default|GetArrow)))))
              (bind _returnvalue_3 (Effects|SpawnEmitterAttached "/Game/Game/Particles/P_ElectricityShot.P_ElectricityShot" (Variables|Default|GetArrow) "None" "0, 0,-40.000000" "0, 0, 0" "SnapToTarget"))
              (Class|ParticleSystemComponent|SetBeamTargetPoint _returnvalue_3 0 (Transformation|GetActorLocation _array_element))
              (Effects|Components|ParticleSystem|SetColorParameter _returnvalue_3 "ParticleColor" (Variables|Default|GetArcColor))
              (else
                (bind _returnvalue_4 (Effects|SpawnEmitterAttached "/Game/Game/Particles/P_ElectricityShot.P_ElectricityShot" (Variables|Default|GetArrow1) "None" "0, 0,-40.000000" "0, 0, 0" "SnapToTarget"))
                (Class|ParticleSystemComponent|SetBeamTargetPoint _returnvalue_4 0 (Transformation|GetActorLocation _array_element))
                (Effects|Components|ParticleSystem|SetColorParameter _returnvalue_4 "ParticleColor" (Variables|Default|GetArcColor))))
            (Class|DamageIntarface|DoDamage(Message) _array_element (Variables|Default|GetArcDamage) 0 0 "VE_Bullet")))))))

(fn ConstructionScript
  (bind _firstcone (Variables|Default|GetFirstCone))
  (bind _returnvalue (Rendering|Material|GetMaterial _firstcone 0))
  (Class|ParticleSystemComponent|SetBeamTargetPoint (Variables|Default|GetP_BeamFire2) 0 (Transformation|GetWorldLocation (Variables|Default|GetArrow)))
  (bind _returnvalue_2 (Rendering|Material|CreateDynamicMaterialInstance _firstcone 0 _returnvalue :!class /Script/Engine.PrimitiveComponent))
  (bind _returnvalue_3 (Rendering|Material|CreateDynamicMaterialInstance (Variables|Default|GetSecondCone) 0 _returnvalue :!class /Script/Engine.PrimitiveComponent))
  (Rendering|Material|SetVectorParameterValue _returnvalue_3 "Color" (Variables|Default|GetBaseColor) :!class /Script/Engine.MaterialInstanceDynamic)
  (Effects|Components|ParticleSystem|SetColorParameter (Variables|Default|GetP_BeamFire2) "ParticleColor" (Variables|Default|GetArcColor)))