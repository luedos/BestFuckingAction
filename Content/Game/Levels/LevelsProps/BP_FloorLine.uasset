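; Level prop that draws a colored, emissive line along an editable spline, built in the construction script.
; Each spline segment gets its own spline mesh with a dynamic unlit material, plus an optional segment that closes the loop.
; The segment materials are cached in MatArray so SetSplineNewColor can recolor the whole line.
; A separate Cube component receives a dynamic glass material with its color set to zero.
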(event EventBeginPlay)

(event Collision|EventActorBeginOverlap
  (params (OtherActor :type Actor%20Object%20Reference)))

(event EventTick
  (params (DeltaSeconds :type Float%20%28single-precision%29)))

(fn ConstructionScript
  (bind _spline (Variables|Default|GetSpline))
  (bind _spline_2 (Variables|Default|GetSpline))
  (bind _spline_3 (Variables|Default|GetSpline))
  (bind _returnvalue (Spline|GetNumberOfSplinePoints _spline))
  (bind (_location _tangent) (Spline|GetLocationandTangentatSplinePoint _spline_3 0 "Local"))
  (bind _returnvalue_2 (- _returnvalue 1))
  (bind (_location_2 _tangent_2) (Spline|GetLocationandTangentatSplinePoint _spline_3 _returnvalue_2 "Local"))
  (Utilities|FlowControl|Sequence
    (:then_0
      (bind _returnvalue_3 (Rendering|Material|CreateDynamicMaterialInstance (Variables|Default|GetCube) 0 "/Game/Game/Materials/M_Glass.M_Glass" :!class /Script/Engine.PrimitiveComponent))
      (Rendering|Material|SetVectorParameterValue _returnvalue_3 "Color" "(R=0.000000,G=0.000000,B=0.000000,A=0.000000)" :!class /Script/Engine.MaterialInstanceDynamic))
    (:then_1
      (for _index (range 0 (- _returnvalue 2))
        (bind _returnvalue_4 (AddComponent|AddSplineMeshComponent false))
        (Transformation|AttachComponentToComponent _returnvalue_4 _spline_2 "None" "KeepRelative" "KeepRelative" "KeepRelative" true)
        (SplineMesh|SetStartandEnd _returnvalue_4 (.Location (Spline|GetLocationandTangentatSplinePoint _spline _index "Local")) (.Tangent (Spline|GetLocationandTangentatSplinePoint _spline _index "Local")) (.Location (Spline|GetLocationandTangentatSplinePoint _spline (+ _index 1) "Local")) (.Tangent (Spline|GetLocationandTangentatSplinePoint _spline (+ _index 1) "Local")) true :!class /Script/Engine.SplineMeshComponent)
        (bind _returnvalue_5 (Rendering|Material|CreateDynamicMaterialInstance _returnvalue_4 0 "/Game/Game/Materials/M_SimpleUnlit.M_SimpleUnlit" :!class /Script/Engine.PrimitiveComponent))
        (Utilities|Array|Add (Variables|Default|GetMatArray) _returnvalue_5)
        (Rendering|Material|SetVectorParameterValue _returnvalue_5 "Color" (Variables|Default|GetColor) :!class /Script/Engine.MaterialInstanceDynamic)
        (Rendering|Material|SetScalarParameterValue _returnvalue_5 "Emissive" (Variables|Default|GetEmissive) :!class /Script/Engine.MaterialInstanceDynamic))
      (if (Variables|Default|GetCloseLoop)
        (Spline|SetClosedLoop _spline_3 (Variables|Default|GetCloseLoop) true)
        (bind _returnvalue_6 (AddComponent|AddSplineMeshComponent false))
        (Transformation|AttachComponentToComponent _returnvalue_6 _spline_2 "None" "KeepRelative" "KeepRelative" "KeepRelative" true)
        (SplineMesh|SetStartandEnd _returnvalue_6 _location_2 _tangent_2 _location _tangent true :!class /Script/Engine.SplineMeshComponent)
        (bind _returnvalue_7 (Rendering|Material|CreateDynamicMaterialInstance _returnvalue_6 0 "/Game/Game/Materials/M_SimpleUnlit.M_SimpleUnlit" :!class /Script/Engine.PrimitiveComponent))
        (Utilities|Array|Add (Variables|Default|GetMatArray) _returnvalue_7)
        (Rendering|Material|SetVectorParameterValue _returnvalue_7 "Color" (Variables|Default|GetColor) :!class /Script/Engine.MaterialInstanceDynamic)
        (Rendering|Material|SetScalarParameterValue _returnvalue_7 "Emissive" (Variables|Default|GetEmissive) :!class /Script/Engine.MaterialInstanceDynamic)))))

(fn SetSplineNewColor
  (params (InColor :type Linear%20Color%20Structure))
  (Rendering|Material|SetVectorParameterValue (Variables|Default|GetMatArray) "Color" InColor :!class /Script/Engine.MaterialInstanceDynamic)
  (Variables|Default|SetColor InColor))