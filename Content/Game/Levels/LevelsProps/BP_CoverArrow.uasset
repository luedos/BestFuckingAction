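; BP_CoverArrow is a cover point marker that tracks whether an enemy is occupying it.
; Each tick it checks whether EnemyWhichOccupy's blackboard references this arrow as CoverArrow with EnumKey at a specific state.
; On a change it updates occupied status and spawns or destroys an electric beam above the point, apparently a debug marker.
; An unconnected variant that polls GetOccupiedStatus is left unused.
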(event EventTick
  (params (DeltaSeconds :type Float%20%28single-precision%29))
  (bind _returnvalue (Transformation|GetWorldLocation))
  (bind _enemywhichoccupy (Variables|Default|GetEnemyWhichOccupy))
  (Utilities|IsValid _enemywhichoccupy
    (:Is%20Valid
      (Utilities|Casting|CastToEnemy_Char _enemywhichoccupy
        (:then
          (bind _returnvalue_2 (AI|GetAIController _enemywhichoccupy))
          (if (and (== self (AI|Components|Blackboard|GetValueasObject (AI|GetBlackboard _returnvalue_2) (Utilities|Name|MakeLiteralName "CoverArrow"))) (== (Class|BlackboardComponent|GetValueasEnum (AI|GetBlackboard _returnvalue_2) (Utilities|Name|MakeLiteralName "EnumKey")) 3))
            (if (not (Variables|Default|GetOldStatus))
              (Class|CoverArrow|ChangeOccupiedStatus true)
              (Variables|Default|SetOldStatus true)
              (bind _returnvalue_3 (Effects|SpawnEmitteratLocation "/Game/ExampleContent/Effects/ParticleSystems/P_electricity_arc_WOEnding.P_electricity_arc_WOEnding" (Transformation|GetWorldLocation)))
              (bind _output_get (Variables|Default|SetTestParticle _returnvalue_3))
              (Class|ParticleSystemComponent|SetBeamTargetPoint _output_get 0 _returnvalue)
              (Class|ParticleSystemComponent|SetBeamSourcePoint _output_get 0 (+ _returnvalue "0, 0,500.000000")))
            (else
              (if (Variables|Default|GetOldStatus) :!label _label
                (Class|CoverArrow|ChangeOccupiedStatus false)
                (Variables|Default|SetOldStatus false)
                (Components|DestroyComponent (Variables|Default|GetTestParticle))))))
        (:CastFailed
          (goto _label))))
    (:Is%20Not%20Valid
      (goto _label))))