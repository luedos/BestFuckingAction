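; BP_Button is a pickup-style button that bobs on a sine wave and fires event dispatchers when picked up.
; PickUpFunc flashes the color bright, then alternates between FireFirst and FireSecond via a FlipFlop, always using FireFirst if HasSecond is false.
; Tick interpolates the flash back to the base color captured in the construction script, writing it to a dynamic material instance.
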(event EventTick
  (params (DeltaSeconds :type Float%20%28single-precision%29))
  (Transformation|SetRelativeLocation (Variables|Default|GetStaticMesh) (Math|Vector|MakeVector 0.0 0.0 (+ (* (Math|Trig|Sin(Radians) (* (Utilities|Time|GetGameTimeinSeconds) 5.0)) 5e+01) 2e+02)) false false)
  (if (> (Math|Vector|VectorLength (- (Math|Conversions|ToVector(LinearColor) (Variables|Default|GetColor)) (Math|Conversions|ToVector(LinearColor) (Variables|Default|GetColorTo)))) 0.001)
    (CallFunction|SetColorFunc (Class|KismetMathLibrary|CInterpto (Variables|Default|GetColor) (Variables|Default|GetColorTo) DeltaSeconds 8.0))))

(event EventPickUpFunc
  (params (FromChar :type Char%20Pawn%20Object%20Reference))
  (Variables|Default|SetColor (* (Variables|Default|GetColorTo) 5e+01))
  (Utilities|FlowControl|FlipFlop
    (:A
      (Default|CallFireFirst :!label _label))
    (:B
      (if (not (Variables|Default|GetHasSecond))
        (goto _label)
        (else
          (Default|CallFireSecond))))))

(fn ConstructionScript
  (bind _staticmesh (Variables|Default|GetStaticMesh))
  (bind _returnvalue (Rendering|Material|CreateDynamicMaterialInstance _staticmesh 0 (Rendering|Material|GetMaterial _staticmesh 0) :!class /Script/Engine.PrimitiveComponent))
  (bind _output_get (Variables|Default|SetMat _returnvalue))
  (Rendering|Material|SetVectorParameterValue _output_get "Color" (Variables|Default|GetColor) :!class /Script/Engine.MaterialInstanceDynamic)
  (Variables|Default|SetColorTo (Variables|Default|GetColor)))

(fn SetColorFunc
  (params (NewColor :type Linear%20Color%20Structure))
  (bind _output_get (Variables|Default|SetColor NewColor))
  (Rendering|Material|SetVectorParameterValue (Variables|Default|GetMat) "Color" _output_get :!class /Script/Engine.MaterialInstanceDynamic))