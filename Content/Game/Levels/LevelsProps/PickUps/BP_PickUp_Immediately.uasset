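; BP_PickUp_Immediately is a pickup prop with a spinning, bobbing mesh and a colored recharge circle, handling visuals and cooldown but no collection or effect logic.
; Construction and BeginPlay create dynamic materials for both parts and set it active.
; DeactivateFunction dims the mesh and starts a timer that calls SetActive after ReloadTime.
; Tick animates the mesh and, while inactive, drives the circle material's Percent from elapsed reload time.
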(event Custom|DeactivateFunction
  (Variables|Default|SetStartTime (Utilities|Time|GetTimeSeconds))
  (Variables|Default|SetIsActive false)
  (Utilities|Time|SetTimerbyFunctionName self "SetActive" (Variables|Default|GetReloadTime))
  (Rendering|Material|SetVectorParameterValue (Variables|Default|GetMeshMat) "Color" (* (Variables|Default|GetMeshColor) 0.05) :!class /Script/Engine.MaterialInstanceDynamic))

(event EventTick
  (params (DeltaSeconds :type Float%20%28single-precision%29))
  (Transformation|AddRelativeRotation (Variables|Default|GetPickUpMesh) (Math|Rotator|MakeRotator 0.0 0.0 (* DeltaSeconds (Variables|Default|GetSpeedOfRotation))) false false)
  (Transformation|SetRelativeLocation (Variables|Default|GetPickUpMesh) (Math|Vector|MakeVector 0.0 0.0 (+ (* (Math|Trig|Sin(Radians) (* (Utilities|Time|GetTimeSeconds) (Variables|Default|GetVibrationSpeed))) (Variables|Default|GetVibrationHight)) 4e+01)) false false)
  (if (not (Variables|Default|GetIsActive))
    (Rendering|Material|SetScalarParameterValue (Variables|Default|GetCicleMat) "Percent" (/ (- (Utilities|Time|GetTimeSeconds) (Variables|Default|GetStartTime)) (Variables|Default|GetReloadTime)) :!class /Script/Engine.MaterialInstanceDynamic)))

(event EventBeginPlay
  (bind _particlesystem (Variables|Default|GetParticleSystem))
  (bind _pickupmesh (Variables|Default|GetPickUpMesh))
  (bind _returnvalue (Rendering|Material|CreateDynamicMaterialInstance _particlesystem 0 (Rendering|Material|GetMaterial _particlesystem 0) :!class /Script/Engine.PrimitiveComponent))
  (bind _output_get (Variables|Default|SetCicleMat _returnvalue))
  (Rendering|Material|SetVectorParameterValue _output_get "Color" (Variables|Default|GetCicleColor) :!class /Script/Engine.MaterialInstanceDynamic)
  (bind _returnvalue_2 (Rendering|Material|CreateDynamicMaterialInstance _pickupmesh 0 (Rendering|Material|GetMaterial _pickupmesh 0) :!class /Script/Engine.PrimitiveComponent))
  (Variables|Default|SetMeshMat _returnvalue_2)
  (CallFunction|SetActive))

(fn ConstructionScript
  (bind _pickupmesh (Variables|Default|GetPickUpMesh))
  (bind _particlesystem (Variables|Default|GetParticleSystem))
  (bind _returnvalue (Rendering|Material|CreateDynamicMaterialInstance _particlesystem 0 (Rendering|Material|GetMaterial _particlesystem 0) :!class /Script/Engine.PrimitiveComponent))
  (bind _output_get (Variables|Default|SetCicleMat _returnvalue))
  (Rendering|Material|SetScalarParameterValue _output_get "Percent" (Variables|Default|GetPercent) :!class /Script/Engine.MaterialInstanceDynamic)
  (Rendering|Material|SetVectorParameterValue _output_get "Color" (Variables|Default|GetCicleColor) :!class /Script/Engine.MaterialInstanceDynamic)
  (bind _returnvalue_2 (Rendering|Material|CreateDynamicMaterialInstance _pickupmesh 0 (Rendering|Material|GetMaterial _pickupmesh 0) :!class /Script/Engine.PrimitiveComponent))
  (bind _output_get_2 (Variables|Default|SetMeshMat _returnvalue_2))
  (Rendering|Material|SetVectorParameterValue _output_get_2 "Color" (Variables|Default|GetMeshColor) :!class /Script/Engine.MaterialInstanceDynamic)
  (CallFunction|SetActive))

(fn SetActive
  (Variables|Default|SetIsActive true)
  (Rendering|Material|SetScalarParameterValue (Variables|Default|GetCicleMat) "Percent" 1.0 :!class /Script/Engine.MaterialInstanceDynamic)
  (Rendering|Material|SetVectorParameterValue (Variables|Default|GetMeshMat) "Color" (Variables|Default|GetMeshColor) :!class /Script/Engine.MaterialInstanceDynamic))