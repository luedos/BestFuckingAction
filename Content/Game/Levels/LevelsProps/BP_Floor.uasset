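; BP_Floor is a scalable, colored cube prop that fades out while an MC_Char overlaps it and fades back in afterward.
; Floors sharing a FloorIndex act as a group, found via GetAllActorsOfClass, changing target alpha only if no other member is overlapped.
; Construction creates a dynamic material for Color.
; When ChangeAlpha is set, Tick interpolates that color's alpha toward the target.
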(event OnComponentBeginOverlap(Cube)
  (params (OverlappedComponent :type Primitive%20Component%20Object%20Reference) (OtherActor :type Actor%20Object%20Reference) (OtherComp :type Primitive%20Component%20Object%20Reference) (OtherBodyIndex :type Integer) (bFromSweep :type Boolean) (SweepResult :type Hit%20Result%20Structure%20%28by%20ref%29))
  (bind _asmc_char (Utilities|Casting|CastToMC_Char OtherActor))
  (if (> (Variables|Default|GetAlpha) 0.5)
    (Utilities|Array|Clear (Variables|Default|GetArray))
    (Variables|Default|SetFindSome false)
    (bind _outactors (Actor|GetAllActorsOfClass "BP_Floor_C"))
    (bind _array_element (Utilities|Array|ForEachLoopwithBreak _outactors :!label _label)
      (:LoopBody
        (if (and (!= self _array_element) (== (Variables|Default|GetFloorIndex) (Variables|BP_Floor_C|GetFloorIndex _array_element)))
          (if (> (Utilities|Array|Length (Collision|GetOverlappingActors (Variables|BP_Floor_C|GetCube _array_element) (Utilities|GetClass _asmc_char) :!class /Script/Engine.PrimitiveComponent)) 0)
            (Variables|Default|SetFindSome true)
            (goto _label Break)
            (else
              (Utilities|Array|Add (Variables|Default|GetArray) _array_element)))))
      (:Completed
        (if (not (Variables|Default|GetFindSome))
          (Utilities|Array|Add (Variables|Default|GetArray) self)
          (CallFunction|SetAlpha (Variables|Default|GetArray) 0.0))))))

(event OnComponentEndOverlap(Cube)
  (params (OverlappedComponent :type Primitive%20Component%20Object%20Reference) (OtherActor :type Actor%20Object%20Reference) (OtherComp :type Primitive%20Component%20Object%20Reference) (OtherBodyIndex :type Integer))
  (bind _array (Variables|Default|GetArray))
  (bind _asmc_char (Utilities|Casting|CastToMC_Char OtherActor))
  (if (< (Variables|Default|GetAlpha) 0.5)
    (Utilities|Array|Clear (Variables|Default|GetArray))
    (Variables|Default|SetFindSome false)
    (bind _outactors (Actor|GetAllActorsOfClass "BP_Floor_C"))
    (bind _array_element (Utilities|Array|ForEachLoopwithBreak _outactors :!label _label)
      (:LoopBody
        (if (and (!= self _array_element) (== (Variables|Default|GetFloorIndex) (Variables|BP_Floor_C|GetFloorIndex _array_element)))
          (if (> (Utilities|Array|Length (Collision|GetOverlappingActors (Variables|BP_Floor_C|GetCube _array_element) (Utilities|GetClass _asmc_char) :!class /Script/Engine.PrimitiveComponent)) 0)
            (Variables|Default|SetFindSome true)
            (goto _label Break)
            (else
              (Utilities|Array|Add (Variables|Default|GetArray) _array_element)))))
      (:Completed
        (if (not (Variables|Default|GetFindSome))
          (Utilities|Array|Add _array self)
          (CallFunction|SetAlpha _array 1.0))))))

(event EventBeginPlay)

(event EventTick
  (params (DeltaSeconds :type Float%20%28single-precision%29))
  (bind _color (Variables|Default|GetColor))
  (if (Variables|Default|GetChangeAlpha)
    (if (not (Math|Float|NearlyEqual(Float) (Variables|Default|GetAlpha) (.a _color) 0.001))
      (CallFunction|SetColorAlpha (Math|Interpolation|FInterpTo (.a _color) (Variables|Default|GetAlpha) DeltaSeconds 1e+01)))))

(fn ConstructionScript
  (bind _cube (Variables|Default|GetCube))
  (Transformation|SetWorldScale3D _cube (Variables|Default|GetScale))
  (bind _returnvalue (Rendering|Material|CreateDynamicMaterialInstance _cube 0 (Rendering|Material|GetMaterial _cube 0) :!class /Script/Engine.PrimitiveComponent))
  (bind _output_get (Variables|Default|SetMAt _returnvalue))
  (Rendering|Material|SetVectorParameterValue _output_get "Color" (Variables|Default|GetColor) :!class /Script/Engine.MaterialInstanceDynamic)
  (if (Variables|Default|GetChangeAlpha)
    (Variables|Default|SetAlpha (.a (Variables|Default|GetColor)))))

(fn SetColorAlpha
  (params (InAlpha :type Float%20%28single-precision%29))
  (Variables|Default|SetColor (Utilities|Struct|MakeLinearColor (.r (Variables|Default|GetColor)) (.g (Variables|Default|GetColor)) (.b (Variables|Default|GetColor)) InAlpha))
  (Rendering|Material|SetVectorParameterValue (Variables|Default|GetMAt) "Color" (Variables|Default|GetColor) :!class /Script/Engine.MaterialInstanceDynamic))

(fn SetAlpha
  (params (InAlpha :type Float%20%28single-precision%29))
  (Variables|Default|SetAlpha InAlpha))