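; Energy gate level prop: two posts joined by three beam effects, with a box that blocks pawns while the gate is closed.
; The construction script sizes post spacing and box from Size, tints posts and beams, and stretches each beam between matching post sockets.
; CloseElGate activates the beams and blocks pawns, while OpenElGate deactivates them and sets overlap.
; StartClosed picks the initial state in construction and at BeginPlay.
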(event EventBeginPlay
  (bind _eltop (Variables|Default|GetElTop))
  (bind _returnvalue (Rendering|Material|GetMaterial _eltop 0))
  (bind _returnvalue_2 (Rendering|Material|CreateDynamicMaterialInstance _eltop 0 _returnvalue :!class /Script/Engine.PrimitiveComponent))
  (bind _returnvalue_3 (Rendering|Material|CreateDynamicMaterialInstance (Variables|Default|GetElMiddle) 0 _returnvalue :!class /Script/Engine.PrimitiveComponent))
  (bind _returnvalue_4 (Rendering|Material|CreateDynamicMaterialInstance (Variables|Default|GetElBottom) 0 _returnvalue :!class /Script/Engine.PrimitiveComponent))
  (Rendering|Material|SetVectorParameterValue _returnvalue_4 "Color" (Variables|Default|GetBeamColor) :!class /Script/Engine.MaterialInstanceDynamic)
  (if (Variables|Default|GetStartClosed)
    (CallFunction|CloseElGate)
    (else
      (CallFunction|OpenElGate))))

(fn ConstructionScript
  (bind _leftmesh (Variables|Default|GetLeftMesh))
  (bind _box (Variables|Default|GetBox))
  (bind _eltop (Variables|Default|GetElTop))
  (bind _rightmesh (Variables|Default|GetRightMesh))
  (bind _leftmesh_2 (Variables|Default|GetLeftMesh))
  (bind _rightmesh_2 (Variables|Default|GetRightMesh))
  (bind _returnvalue (Rendering|Material|GetMaterial _eltop 0))
  (bind _boxextent (Variables|/Script/Engine.BoxComponent|GetBoxExtent _box))
  (Transformation|SetRelativeLocation (Variables|Default|GetRightMesh) (Math|Vector|MakeVector 0.0 (/ (Variables|Default|GetSize) 2.0) 0.0) false false)
  (Transformation|SetRelativeLocation (Variables|Default|GetLeftMesh) (Math|Vector|MakeVector 0.0 (/ (Variables|Default|GetSize) -2.0) 0.0) false false)
  (Components|Box|SetBoxExtent _box (Math|Vector|MakeVector (.x _boxextent) (/ (Variables|Default|GetSize) 2.0) (.z _boxextent)) true)
  (bind _returnvalue_2 (Rendering|Material|CreateDynamicMaterialInstance _rightmesh_2 0 (Rendering|Material|GetMaterial _rightmesh_2 0) :!class /Script/Engine.PrimitiveComponent))
  (bind _returnvalue_3 (Rendering|Material|CreateDynamicMaterialInstance _leftmesh 0 (Rendering|Material|GetMaterial _leftmesh 0) :!class /Script/Engine.PrimitiveComponent))
  (Rendering|Material|SetVectorParameterValue _returnvalue_3 "Color" (Variables|Default|GetColor) :!class /Script/Engine.MaterialInstanceDynamic)
  (Transformation|AttachComponentToComponent (Variables|Default|GetElTop) _rightmesh "TopSocket" "SnapToTarget" "SnapToTarget" "KeepRelative" true)
  (Transformation|AttachComponentToComponent (Variables|Default|GetElMiddle) _rightmesh "MiddleSocket" "SnapToTarget" "SnapToTarget" "KeepRelative" true)
  (Transformation|AttachComponentToComponent (Variables|Default|GetElBottom) _rightmesh "BottomSocket" "SnapToTarget" "SnapToTarget" "KeepRelative" true)
  (Class|ParticleSystemComponent|SetBeamTargetPoint (Variables|Default|GetElTop) 0 (Transformation|GetSocketLocation _leftmesh_2 "TopSocket"))
  (Class|ParticleSystemComponent|SetBeamTargetPoint (Variables|Default|GetElMiddle) 0 (Transformation|GetSocketLocation _leftmesh_2 "MiddleSocket"))
  (Class|ParticleSystemComponent|SetBeamTargetPoint (Variables|Default|GetElBottom) 0 (Transformation|GetSocketLocation _leftmesh_2 "BottomSocket"))
  (bind _returnvalue_4 (Rendering|Material|CreateDynamicMaterialInstance _eltop 0 _returnvalue :!class /Script/Engine.PrimitiveComponent))
  (bind _returnvalue_5 (Rendering|Material|CreateDynamicMaterialInstance (Variables|Default|GetElMiddle) 0 _returnvalue :!class /Script/Engine.PrimitiveComponent))
  (bind _returnvalue_6 (Rendering|Material|CreateDynamicMaterialInstance (Variables|Default|GetElBottom) 0 _returnvalue :!class /Script/Engine.PrimitiveComponent))
  (Rendering|Material|SetVectorParameterValue _returnvalue_6 "Color" (Variables|Default|GetBeamColor) :!class /Script/Engine.MaterialInstanceDynamic)
  (if (Variables|Default|GetStartClosed)
    (CallFunction|CloseElGate)
    (else
      (CallFunction|OpenElGate))))

(fn OpenElGate
  (Components|Activation|SetActive (Variables|Default|GetElBottom) false true)
  (Collision|SetCollisionResponsetoChannel (Variables|Default|GetBox) "ECC_Pawn" "ECR_Overlap"))

(fn CloseElGate
  (bind _leftmesh (Variables|Default|GetLeftMesh))
  (Components|Activation|SetActive (Variables|Default|GetElBottom) true true)
  (Collision|SetCollisionResponsetoChannel (Variables|Default|GetBox) "ECC_Pawn" "ECR_Block")
  (Class|ParticleSystemComponent|SetBeamTargetPoint (Variables|Default|GetElTop) 0 (Transformation|GetSocketLocation _leftmesh "TopSocket"))
  (Class|ParticleSystemComponent|SetBeamTargetPoint (Variables|Default|GetElMiddle) 0 (Transformation|GetSocketLocation _leftmesh "MiddleSocket"))
  (Class|ParticleSystemComponent|SetBeamTargetPoint (Variables|Default|GetElBottom) 0 (Transformation|GetSocketLocation _leftmesh "BottomSocket")))