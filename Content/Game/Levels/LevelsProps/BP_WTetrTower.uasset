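; Destructible tower prop that periodically links electric arc beams to nearby BP_Enemy_WTetrahdron enemies and triggers their rays.
; Sphere overlap registers enemies, and Tick prunes invalid or out-of-range ones.
; Despite its name, Get2Random gathers ray-ready enemies in random order without capping at two; each receives a beam via StartRay.
; RayTimeLine animates beam noise and color, then a random delay re-arms the tower.
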(event OnComponentBeginOverlap(Sphere)
  (params (OverlappedComponent :type Primitive%20Component%20Object%20Reference) (OtherActor :type Actor%20Object%20Reference) (OtherComp :type Primitive%20Component%20Object%20Reference) (OtherBodyIndex :type Integer) (bFromSweep :type Boolean) (SweepResult :type Hit%20Result%20Structure%20%28by%20ref%29))
  (bind _asbp_enemy_wtetrahdron (Utilities|Casting|CastToBP_Enemy_WTetrahdron OtherActor))
  (Utilities|Array|AddUnique (Variables|Default|GetWT_Array) _asbp_enemy_wtetrahdron))

(event EventBeginPlay)

(event Collision|EventActorBeginOverlap
  (params (OtherActor :type Actor%20Object%20Reference)))

(event EventDoDamage
  (params (Damage :type Float%20%28single-precision%29) (CallInstigator :type Player%20Controller%20Object%20Reference) (Couser :type Actor%20Object%20Reference) (DamageType :type EDamageType%20Enum :default "VE_Bullet"))
  (bind _output_get (Variables|Default|SetHP (- (stale _output_get) Damage)))
  (if (< _output_get 0.0)
    (Actor|DestroyActor)))

(event EventTick
  (params (DeltaSeconds :type Float%20%28single-precision%29))
  (if (> (Utilities|Array|Length (Variables|Default|GetWT_Array)) 0)
    (CallFunction|CheckArray)
    (if (Variables|Default|GetCanRaySpawn)
      (Variables|Default|SetCanRaySpawn false)
      (bind _outarray (CallFunction|Get2Random))
      (Utilities|Array|Clear (Variables|Default|GetParticleArray))
      (for _array_element _outarray
        (bind _returnvalue (Effects|SpawnEmitteratLocation "/Game/Game/Particles/P_ElectrisityLongShot.P_ElectrisityLongShot" (Transformation|GetWorldLocation (Variables|Default|GetParticleSystem))))
        (Effects|Components|ParticleSystem|SetColorParameter _returnvalue "ParticleColor" (Variables|Default|GetArcColor))
        (Class|ParticleSystemComponent|SetBeamTargetPoint _returnvalue 0 (Transformation|GetActorLocation _array_element))
        (Utilities|Array|Add (Variables|Default|GetParticleArray) _returnvalue)
        (Class|EnemyWTetrahdron|StartRay _array_element 1.1 2.2 _returnvalue))
      (bind _newtrack_0 (Timeline|RayTimeLine PlayFromStart)
        (:Update
          (CallFunction|SetParticlesValues (+ (/ _newtrack_0 2.0) 0.75) (* (Variables|Default|GetArcColor) (+ _newtrack_0 1.0))))
        (:Finished
          (Utilities|FlowControl|Delay (Math|Random|RandomFloatinRange 0.5 1.3))
          (Variables|Default|SetCanRaySpawn true))))))

(fn ConstructionScript
  (bind _mesh (Variables|Default|GetMesh))
  (bind _returnvalue (Rendering|Material|CreateDynamicMaterialInstance _mesh 0 (Rendering|Material|GetMaterial _mesh 0) :!class /Script/Engine.PrimitiveComponent))
  (Rendering|Material|SetVectorParameterValue _returnvalue "Color" (Variables|Default|GetBaseColor) :!class /Script/Engine.MaterialInstanceDynamic)
  (Effects|Components|ParticleSystem|SetColorParameter (Variables|Default|GetParticleSystem) "ParticleColor" (Variables|Default|GetArcColor)))

(fn CheckArray
  (bind _sphere (Variables|Default|GetSphere))
  (for _array_element (Variables|Default|GetWT_Array)
    (Utilities|IsValid _array_element
      (:Is%20Valid
        (if (> (Math|Vector|VectorLength (- (Transformation|GetActorLocation _array_element) (Transformation|GetWorldLocation _sphere))) (+ (Variables|/Script/Engine.SphereComponent|GetSphereRadius _sphere) 25.0))
          (Utilities|Array|RemoveItem (Variables|Default|GetWT_Array) _array_element :!label _label)))
      (:Is%20Not%20Valid
        (goto _label)))))

(fn Get2Random
  (bind _wt_array (Variables|Default|GetWT_Array))
  (LocalVariables|SetLocalInArray _wt_array)
  (Utilities|FlowControl|ForLoopwithBreak 0 (Utilities|Array|LastIndex _wt_array) :!label _label
    (:LoopBody
      (if (> (Utilities|Array|Length (LocalVariables|GetLocalInArray)) 0)
        (LocalVariables|SetLocalActor (Utilities|Array|Get(acopy) (LocalVariables|GetLocalInArray) (Math|Random|RandomInteger (Utilities|Array|LastIndex (LocalVariables|GetLocalInArray)))))
        (if (Class|EnemyWTetrahdron|GetIsCanRay (LocalVariables|GetLocalActor))
          (Utilities|Array|Add (LocalVariables|GetLocalOutArray) (LocalVariables|GetLocalActor)))
        (Utilities|Array|RemoveItem (LocalVariables|GetLocalInArray) (LocalVariables|GetLocalActor))
        (else
          (goto _label Break))))
    (:Completed
      (return (LocalVariables|GetLocalOutArray)))))

(fn SetParticlesValues
  (params (NoiseIn :type Float%20%28single-precision%29) (ColorIn :type Linear%20Color%20Structure))
  (bind _particlearray (Variables|Default|GetParticleArray))
  (for _array_element _particlearray
    (Utilities|IsValid _array_element
      (:Is%20Valid
        (Effects|Components|ParticleSystem|SetFloatParameter _array_element "NoseScale" NoiseIn)
        (Effects|Components|ParticleSystem|SetColorParameter _array_element "ParticleColor" ColorIn))
      (:Is%20Not%20Valid
        (Utilities|Array|RemoveItem _particlearray _array_element)))))