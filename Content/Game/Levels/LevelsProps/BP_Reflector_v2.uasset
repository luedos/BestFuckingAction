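; BP_Reflector_v2 is a level prop that forms a resizable, colored reflector panel, set up entirely in the Construction Script.
; The Squere variable sets the Y and Z extents of a box component, keeping its X depth.
; Cube1 scales to match that box as a very thin slab.
; A dynamic material instance on the cube receives the Color variable, and no gameplay logic runs.
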(event EventBeginPlay)

(event Collision|EventActorBeginOverlap
  (params (OtherActor :type Actor%20Object%20Reference)))

(event EventTick
  (params (DeltaSeconds :type Float%20%28single-precision%29)))

(fn ConstructionScript
  (bind _boxcomponent (Variables|Default|GetBoxComponent))
  (bind _cube1 (Variables|Default|GetCube1))
  (bind _squere (Variables|Default|GetSquere))
  (bind _boxextent (Variables|/Script/Engine.BoxComponent|GetBoxExtent _boxcomponent))
  (bind _returnvalue (* _boxextent 0.02))
  (Components|Box|SetBoxExtent _boxcomponent (Math|Vector|MakeVector (.x (Variables|/Script/Engine.BoxComponent|GetBoxExtent _boxcomponent)) (.x _squere) (.y _squere)) true)
  (Transformation|SetWorldScale3D _cube1 (Math|Vector|MakeVector 0.01 (.y _returnvalue) (.z _returnvalue)))
  (bind _returnvalue_2 (Rendering|Material|CreateDynamicMaterialInstance _cube1 0 (Rendering|Material|GetMaterial _cube1 0) :!class /Script/Engine.PrimitiveComponent))
  (Rendering|Material|SetVectorParameterValue _returnvalue_2 "Color" (Variables|Default|GetColor) :!class /Script/Engine.MaterialInstanceDynamic))