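; Configurable cover block for levels, built in the construction script from a scaled cube with a tinted glass or simple-color material.
; It spaces BP_CoverArrow components along the X length on the optional front and back sides, storing them in ArrowArray.
; An optional eight-point spline traces a rounded rectangle around the cube, rendered as a closed loop of emissive spline meshes.
; Their dynamic materials are cached so SetSplineNewColor can recolor the outline.
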(event EventBeginPlay)

(event Collision|EventActorBeginOverlap
  (params (OtherActor :type Actor%20Object%20Reference)))

(event EventTick
  (params (DeltaSeconds :type Float%20%28single-precision%29)))

(fn ConstructionScript
  (bind _glass_simple (Variables|Cube|GetGlass/Simple))
  (bind _splineheight (Variables|Spline|GetSplineHeight))
  (bind _cubescale (Variables|Cube|GetCubeScale))
  (bind _cubescale_2 (Variables|Cube|GetCubeScale))
  (bind _cubescale_3 (Variables|Cube|GetCubeScale))
  (bind _arrowarray (Variables|Default|GetArrowArray))
  (bind _splineheight_2 (Variables|Spline|GetSplineHeight))
  (bind _splineheight_3 (Variables|Spline|GetSplineHeight))
  (bind _cube (Variables|Default|GetCube))
  (bind _spline (Variables|Default|GetSpline))
  (bind _spline_2 (Variables|Default|GetSpline))
  (bind _spline_3 (Variables|Default|GetSpline))
  (bind _splinetangent (Variables|Spline|GetSplineTangent))
  (bind _cubescale_4 (Variables|Cube|GetCubeScale))
  (bind _returnvalue (Spline|GetNumberOfSplinePoints _spline))
  (bind _returnvalue_2 (/ _cubescale_4 0.02))
  (bind (_location _tangent) (Spline|GetLocationandTangentatSplinePoint _spline 0 "Local"))
  (bind _returnvalue_3 (* _cubescale_2 1e+02))
  (bind _returnvalue_4 (/ _cubescale_3 0.02))
  (bind _returnvalue_5 (Math|Float|Floor (.x _cubescale)))
  (bind _returnvalue_6 (* _splinetangent -1.0))
  (bind _returnvalue_7 (/ (.y _returnvalue_3) 2.0))
  (bind _returnvalue_8 (- (.x _returnvalue_4) _splineheight_2))
  (bind _returnvalue_9 (- (.y _returnvalue_4) _splineheight_3))
  (bind _returnvalue_10 (- _returnvalue 1))
  (bind _returnvalue_11 (== _returnvalue_5 0))
  (bind _returnvalue_12 (- _returnvalue_5 1))
  (bind _returnvalue_13 (+ (.y _returnvalue_4) _splineheight_3))
  (bind _returnvalue_14 (+ (.x _returnvalue_4) _splineheight_2))
  (bind (_location_2 _tangent_2) (Spline|GetLocationandTangentatSplinePoint _spline _returnvalue_10 "Local"))
  (bind _returnvalue_15 (Math|Float|Clamp(Float) _returnvalue_8 0.0 1e+04))
  (bind _returnvalue_16 (Math|Float|Clamp(Float) _returnvalue_9 0.0 1e+04))
  (bind _returnvalue_17 (+ _returnvalue_7 5e+01))
  (bind _returnvalue_18 (* _returnvalue_14 -1.0))
  (bind _returnvalue_19 (* _returnvalue_13 -1.0))
  (bind _returnvalue_20 (select _returnvalue_11 _returnvalue_5 _returnvalue_12))
  (bind _returnvalue_21 (* _returnvalue_15 -1.0))
  (bind _returnvalue_22 (* _returnvalue_16 -1.0))
  (Utilities|FlowControl|Sequence
    (:then_0
      (Transformation|SetWorldScale3D _cube (Variables|Cube|GetCubeScale))
      (if _glass_simple
        (bind _returnvalue_23 (Rendering|Material|CreateDynamicMaterialInstance "/Game/Game/Materials/M_Glass_Inst.M_Glass_Inst" :!class /Script/Engine.KismetMaterialLibrary))
        (else
          (bind _returnvalue_24 (Rendering|Material|CreateDynamicMaterialInstance "/Game/Game/Materials/M_SimpleColor.M_SimpleColor" :!class /Script/Engine.KismetMaterialLibrary))))
      (Rendering|Material|SetMaterial _cube 0 (select _glass_simple _returnvalue_23 _returnvalue_24))
      (Rendering|Material|SetVectorParameterValue (select _glass_simple _returnvalue_23 _returnvalue_24) "Color" (Variables|Cube|GetColor) :!class /Script/Engine.MaterialInstanceDynamic)
      (for _index (range 0 _returnvalue_20)
        (if (Variables|Cube|GetUseFront)
          (bind _returnvalue_25 (AddComponent|AddBPCoverArrow false (Math|Transform|MakeTransform (Math|Vector|MakeVector (* (+ (Math|Conversions|ToFloat(Integer) _index) (* (/ (Math|Conversions|ToFloat(Integer) _returnvalue_20) 2.0) -1.0)) 1e+02) _returnvalue_17 4e+01) "90.000000, 0, 0" "1,1,1")))
          (Utilities|Array|Add _arrowarray _returnvalue_25))
        (if (Variables|Cube|GetUseBack)
          (bind _returnvalue_26 (AddComponent|AddBPCoverArrow false (Math|Transform|MakeTransform (Math|Vector|MakeVector (* (+ (Math|Conversions|ToFloat(Integer) _index) (* (/ (Math|Conversions|ToFloat(Integer) _returnvalue_20) 2.0) -1.0)) 1e+02) (* _returnvalue_17 -1.0) 4e+01) "90.000000, 0, 0" "1,1,1")))
          (Utilities|Array|Add _arrowarray _returnvalue_26))))
    (:then_1
      (if (Variables|Spline|GetUseSpline)
        (Variables|Default|SetPointLoc (Math|Vector2D|MakeVector2D (Math|Float|Clamp(Float) (- (.x _returnvalue_2) _splineheight) 0.0 1e+04) (+ (.y _returnvalue_2) _splineheight)))
        (Variables|Default|SetPointTan (Math|Vector2D|MakeVector2D (* (Variables|Spline|GetSplineTangent) -1.0) 0.0))
        (Spline|ClearSplinePoints (Variables|Default|GetSpline) true)
        (for _index_2 (range 0 7)
          (Spline|AddSplinePoint _spline_3 (Math|Vector|MakeVector (.x (Variables|Default|GetPointLoc)) (.y (Variables|Default|GetPointLoc)) 0.0) "Local" true)
          (Spline|SetTangentatSplinePoint _spline_3 _index_2 (Math|Vector|MakeVector (.x (Variables|Default|GetPointTan)) (.y (Variables|Default|GetPointTan)) 0.0) "Local" true)
          (switch int _index_2
            (:0
              (Variables|Default|SetPointLoc (Math|Vector2D|MakeVector2D _returnvalue_21 _returnvalue_13))
              (Variables|Default|SetPointTan (Math|Vector2D|MakeVector2D _returnvalue_6 0.0)))
            (:1
              (Variables|Default|SetPointLoc (Math|Vector2D|MakeVector2D _returnvalue_18 _returnvalue_16))
              (Variables|Default|SetPointTan (Math|Vector2D|MakeVector2D 0.0 _returnvalue_6)))
            (:2
              (Variables|Default|SetPointLoc (Math|Vector2D|MakeVector2D _returnvalue_18 _returnvalue_22))
              (Variables|Default|SetPointTan (Math|Vector2D|MakeVector2D 0.0 _returnvalue_6)))
            (:3
              (Variables|Default|SetPointLoc (Math|Vector2D|MakeVector2D _returnvalue_21 _returnvalue_19))
              (Variables|Default|SetPointTan (Math|Vector2D|MakeVector2D _splinetangent 0.0)))
            (:4
              (Variables|Default|SetPointLoc (Math|Vector2D|MakeVector2D _returnvalue_15 _returnvalue_19))
              (Variables|Default|SetPointTan (Math|Vector2D|MakeVector2D _splinetangent 0.0)))
            (:5
              (Variables|Default|SetPointLoc (Math|Vector2D|MakeVector2D _returnvalue_14 _returnvalue_22))
              (Variables|Default|SetPointTan (Math|Vector2D|MakeVector2D 0.0 _splinetangent)))
            (:6
              (Variables|Default|SetPointLoc (Math|Vector2D|MakeVector2D _returnvalue_14 _returnvalue_16))
              (Variables|Default|SetPointTan (Math|Vector2D|MakeVector2D 0.0 _splinetangent)))))
        (for _index_3 (range 0 (- _returnvalue 2))
          (bind _returnvalue_27 (AddComponent|AddSplineMeshComponent false))
          (Transformation|AttachComponentToComponent _returnvalue_27 _spline_2 "None" "KeepRelative" "KeepRelative" "KeepRelative" true)
          (SplineMesh|SetStartandEnd _returnvalue_27 (.Location (Spline|GetLocationandTangentatSplinePoint _spline _index_3 "Local")) (.Tangent (Spline|GetLocationandTangentatSplinePoint _spline _index_3 "Local")) (.Location (Spline|GetLocationandTangentatSplinePoint _spline (+ _index_3 1) "Local")) (.Tangent (Spline|GetLocationandTangentatSplinePoint _spline (+ _index_3 1) "Local")) true :!class /Script/Engine.SplineMeshComponent)
          (bind _returnvalue_28 (Rendering|Material|CreateDynamicMaterialInstance _returnvalue_27 0 "/Game/Game/Materials/M_SimpleUnlit.M_SimpleUnlit" :!class /Script/Engine.PrimitiveComponent))
          (Utilities|Array|Add (Variables|Default|GetMatArray) _returnvalue_28)
          (Rendering|Material|SetVectorParameterValue _returnvalue_28 "Color" (Variables|Spline|GetSplineColor) :!class /Script/Engine.MaterialInstanceDynamic)
          (Rendering|Material|SetScalarParameterValue _returnvalue_28 "Emissive" (Variables|Spline|GetSlineEmissive) :!class /Script/Engine.MaterialInstanceDynamic))
        (bind _returnvalue_29 (AddComponent|AddSplineMeshComponent false))
        (Transformation|AttachComponentToComponent _returnvalue_29 _spline_2 "None" "KeepRelative" "KeepRelative" "KeepRelative" true)
        (SplineMesh|SetStartandEnd _returnvalue_29 _location_2 _tangent_2 _location _tangent true :!class /Script/Engine.SplineMeshComponent)
        (bind _returnvalue_30 (Rendering|Material|CreateDynamicMaterialInstance _returnvalue_29 0 "/Game/Game/Materials/M_SimpleUnlit.M_SimpleUnlit" :!class /Script/Engine.PrimitiveComponent))
        (Utilities|Array|Add (Variables|Default|GetMatArray) _returnvalue_30)
        (Rendering|Material|SetVectorParameterValue _returnvalue_30 "Color" (Variables|Spline|GetSplineColor) :!class /Script/Engine.MaterialInstanceDynamic)
        (Rendering|Material|SetScalarParameterValue _returnvalue_30 "Emissive" (Variables|Spline|GetSlineEmissive) :!class /Script/Engine.MaterialInstanceDynamic)))))

(fn SetSplineNewColor
  (params (Color :type Linear%20Color%20Structure))
  (Rendering|Material|SetVectorParameterValue (Variables|Default|GetMatArray) "Color" Color :!class /Script/Engine.MaterialInstanceDynamic)
  (Variables|Spline|SetSplineColor Color))