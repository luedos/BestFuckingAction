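; Team-aware energy ball projectile that lobs in an arc toward a target point and explodes for area damage.
; BeginPlay computes the launch velocity and starts a power-up sound and fuse, while Tick pulses and grows the sphere, shifting its color toward red.
; It detonates on fuse expiry or on overlapping a damageable non-teammate.
; The blast sphere-traces for targets, then line-traces each to apply distance-scaled damage through DamageIntarface, tracking already-hit actors and components.
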(event OnComponentBeginOverlap(Sphere2)
  (params (OverlappedComponent :type Primitive%20Component%20Object%20Reference) (OtherActor :type Actor%20Object%20Reference) (OtherComp :type Primitive%20Component%20Object%20Reference) (OtherBodyIndex :type Integer) (bFromSweep :type Boolean) (SweepResult :type Hit%20Result%20Structure%20%28by%20ref%29))
  (if (Utilities|DoesObjectImplementInterface OtherActor "/Script/Demo_001.DamageIntarface")
    (bind _aschar_pawn (Utilities|Casting|CastToCharPawn OtherActor)
      (:then
        (if (!= (Class|CharPawn|GetTeam _aschar_pawn) (Variables|Default|GetProjectailTeam))
          (CallFunction|Expload&Destroy)))
      (:CastFailed
        (CallFunction|Expload&Destroy :!label _label)))
    (elif (Utilities|DoesObjectImplementInterface OtherComp "/Script/Demo_001.DamageIntarface")
      (goto _label))))

(event Custom|Expload&Destroy
  (bind _powerupsound (Variables|Default|GetPowerUpSound))
  (CallFunction|Expload)
  (Utilities|IsValid _powerupsound
    (:Is%20Valid
      (Audio|Components|Audio|Stop _powerupsound)
      (Class|Projectail|DestroyProjectailItself (+ (Transformation|GetActorLocation) "0, 0,60.000000")))))

(event EventBeginPlay
  (bind _returnvalue (Audio|SpawnSoundAttached "/Game/Game/Sounds/EnergyBall/S_EnergyBall_PoverUp.S_EnergyBall_PoverUp" (Variables|Default|GetSphere2)))
  (Variables|Default|SetPowerUpSound _returnvalue)
  (bind _velocityout (CallFunction|SetProjVelocity (Variables|Default|GetPointVector)))
  (Variables|/Script/Engine.MovementComponent|SetVelocity (Variables|Default|GetProjectileMovement) _velocityout)
  (Utilities|FlowControl|Delay (Variables|Default|GetExploadDelay))
  (CallFunction|Expload)
  (Utilities|IsValid (Variables|Default|GetPowerUpSound)
    (:Is%20Valid
      (Audio|Components|Audio|Stop (Variables|Default|GetPowerUpSound))
      (Class|Projectail|DestroyProjectailItself (+ (Transformation|GetActorLocation) "0, 0,60.000000")))))

(event Collision|EventActorBeginOverlap
  (params (OtherActor :type Actor%20Object%20Reference)))

(event EventTick
  (params (DeltaSeconds :type Float%20%28single-precision%29))
  (Utilities|FlowControl|Sequence
    (:then_0
      (Transformation|SetWorldScale3D (Variables|Default|GetSphere1) (Math|Conversions|ToVector(Float) (+ (/ (Math|Trig|Sin(Radians) (* (Utilities|Time|GetTimeSeconds) 8.0)) 2.0) 0.7 (Variables|Default|GetScaleValue)))))
    (:then_1
      (Utilities|FlowControl|Delay 0.2)
      (CallFunction|ChangeColor (Math|Color|Lerp(LinearColor) "(R=10.000000,G=10.000000,B=0.200000,A=0.200000)" "(R=20.000000,G=0.000000,B=0.000000,A=1.000000)" (/ (* (Variables|Default|GetCount) 0.2) (Variables|Default|GetExploadDelay))))
      (Math|Integer|IncrementInt (Variables|Default|GetCount)
        (:%20%20
          (bind _output_get (Variables|Default|SetScaleValue (+ (stale _output_get) 0.3))))))))

(fn ConstructionScript
  (bind _returnvalue (Rendering|Material|CreateDynamicMaterialInstance (Variables|Default|GetSphere1) 0 "/Game/Game/Materials/M_Glass.M_Glass" :!class /Script/Engine.PrimitiveComponent))
  (Variables|Default|SetSphereMat _returnvalue)
  (Rendering|Material|SetVectorParameterValue _returnvalue "Color" (Variables|Default|GetColor) :!class /Script/Engine.MaterialInstanceDynamic))

(fn SetProjVelocity
  (params (PointVector :type Vector))
  (bind _returnvalue (Transformation|GetActorLocation))
  (bind _returnvalue_2 (Math|Float|Absolute(Float) 6.86e+03))
  (bind _maxlength (Variables|Default|GetMaxLength))
  (bind _returnvalue_3 (- PointVector _returnvalue))
  (bind _returnvalue_4 (Math|Vector|VectorLength _returnvalue_3))
  (Development|PrintString "")
  (LocalVariables|SetLength (select (> _returnvalue_4 _maxlength) _maxlength _returnvalue_4))
  (LocalVariables|SetYVelocity (Math|Float|Sqrt (* (Variables|Default|GetMaxHeight) _returnvalue_2 2.0)))
  (LocalVariables|SetXVelosity (* (LocalVariables|GetLength) (Math|Float|Sqrt (/ _returnvalue_2 (* (Variables|Default|GetMaxHeight) 2.0))) 0.5))
  (return (+ (* (Math|Vector|MakeVector 0.0 0.0 1.0) (LocalVariables|GetYVelocity)) (* (Math|Rotator|GetRotationXVector (Math|Rotator|MakeRotator 0.0 0.0 (.yaw (Math|Rotator|FindLookatRotation (Transformation|GetActorLocation) (Variables|Default|GetPointVector))))) (LocalVariables|GetXVelosity)))))

(fn Expload
  (bind _returnvalue (Transformation|GetActorLocation))
  (bind _returnvalue_2 (Math|Float|MakeLiteralFloat 1.3e+02))
  (bind _returnvalue_3 (Math|Float|MakeLiteralFloat 4e+01))
  (bind _returnvalue_4 (Transformation|GetActorLocation))
  (bind _self self)
  (bind _projectaildamage (Variables|Default|GetProjectailDamage))
  (bind _projectaildamage_2 (Variables|Default|GetProjectailDamage))
  (bind _outhits (Class|KismetSystemLibrary|SphereTraceMultiNEW _returnvalue_4 (+ _returnvalue_4 "0, 0,1.000000") 1.7e+02 "TraceTypeQuery3" false 0 "ForDuration" true))
  (for _array_element _outhits
    (if (Utilities|DoesObjectImplementInterface (.HitActor (Collision|BreakHitResult _array_element)) "/Script/Demo_001.DamageIntarface")
      (bind _aschar_pawn (Utilities|Casting|CastToCharPawn (.HitActor (Collision|BreakHitResult _array_element)))
        (:then
          (if (!= (Variables|Default|GetProjectailTeam) (Class|CharPawn|GetTeam _aschar_pawn))
            (bind _outhits_2 (Class|KismetSystemLibrary|LineTraceMultiNEW (Transformation|GetActorLocation) (Transformation|GetActorLocation (.HitActor (Collision|BreakHitResult _array_element))) "TraceTypeQuery3" false 0 "None" true :!label _label))
            (bind _array_element_2 (Utilities|Array|ForEachLoopwithBreak _outhits_2 :!label _label_2)
              (:LoopBody
                (if (== (.HitActor (Collision|BreakHitResult _array_element_2)) (.HitActor (Collision|BreakHitResult _array_element)))
                  (if (Utilities|DoesObjectImplementInterface (.HitComponent (Collision|BreakHitResult _array_element_2)) "/Script/Demo_001.DamageIntarface")
                    (if (not (Utilities|Array|ContainsItem (LocalVariables|GetComponents) (.HitComponent (Collision|BreakHitResult _array_element_2))))
                      (Class|DamageIntarface|DoDamage(Message) (.HitComponent (Collision|BreakHitResult _array_element_2)) (+ (* (Math|Float|Clamp(Float) (/ (+ (- _returnvalue_2 (Math|Vector|VectorLength (- (Transformation|GetWorldLocation (.HitComponent (Collision|BreakHitResult _array_element_2))) _returnvalue))) _returnvalue_3) _returnvalue_2)) _projectaildamage_2) _projectaildamage_2) "TE_Enemy" _self "VE_LaserBeam")
                      (Utilities|Array|Add (LocalVariables|GetComponents) (.HitComponent (Collision|BreakHitResult _array_element_2)))
                      (goto _label_2 Break))
                    (elif (not (Utilities|Array|ContainsItem (LocalVariables|GetIgnorActors) (.HitActor (Collision|BreakHitResult _array_element_2))))
                      (Class|DamageIntarface|DoDamage(Message) (.HitActor (Collision|BreakHitResult _array_element_2)) (+ (* (Math|Float|Clamp(Float) (/ (+ (- _returnvalue_2 (Math|Vector|VectorLength (- (Transformation|GetActorLocation (.HitActor (Collision|BreakHitResult _array_element_2))) _returnvalue))) _returnvalue_3) _returnvalue_2)) _projectaildamage_2) _projectaildamage_2) "TE_Enemy" _self "VE_LaserBeam")
                      (Utilities|Array|Add (LocalVariables|GetIgnorActors) (.HitActor (Collision|BreakHitResult _array_element_2)))
                      (goto _label_2 Break))))))))
        (:CastFailed
          (goto _label)))
      (elif (Utilities|DoesObjectImplementInterface (.HitComponent (Collision|BreakHitResult _array_element)) "/Script/Demo_001.DamageIntarface")
        (bind _outhits_3 (Class|KismetSystemLibrary|LineTraceMultiNEW (Transformation|GetActorLocation) (Transformation|GetWorldLocation (.HitComponent (Collision|BreakHitResult _array_element))) "TraceTypeQuery3" false 0 "None" true))
        (bind _array_element_3 (Utilities|Array|ForEachLoopwithBreak _outhits_3 :!label _label_3)
          (:LoopBody
            (if (and (== (.HitComponent (Collision|BreakHitResult _array_element_3)) (.HitComponent (Collision|BreakHitResult _array_element))) (not (Utilities|Array|ContainsItem (LocalVariables|GetComponents) (.HitComponent (Collision|BreakHitResult _array_element)))))
              (Class|DamageIntarface|DoDamage(Message) (.HitComponent (Collision|BreakHitResult _array_element_3)) (+ (* (Math|Float|Clamp(Float) (/ (+ (- _returnvalue_2 (Math|Vector|VectorLength (- (Transformation|GetWorldLocation (.HitComponent (Collision|BreakHitResult _array_element_3))) (Transformation|GetActorLocation)))) _returnvalue_3) _returnvalue_2)) _projectaildamage) _projectaildamage) "TE_Enemy" self "VE_LaserBeam")
              (Utilities|Array|Add (LocalVariables|GetComponents) (.HitComponent (Collision|BreakHitResult _array_element_3)))
              (goto _label_3 Break))))))))

(fn ChangeColor
  (params (InColor :type Linear%20Color%20Structure))
  (Rendering|Material|SetVectorParameterValue (Variables|Default|GetSphereMat) "Color" InColor :!class /Script/Engine.MaterialInstanceDynamic)
  (Variables|Default|SetColor InColor))