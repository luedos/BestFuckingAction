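; BP_BolvanBullet is a weapon projectile that deals bullet damage to the actors it hits.
; On a mesh hit it sends a damage message to the other actor with itself as causer, then destroys itself at the impact location.
; Mesh overlaps are forwarded to a separate damage-after-overlap routine.
; The construction script tints the mesh through a dynamic instance of a simple unlit material using its Color variable.
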(event OnComponentBeginOverlap(ProjectailMesh)
  (params (OverlappedComponent :type Primitive%20Component%20Object%20Reference) (OtherActor :type Actor%20Object%20Reference) (OtherComp :type Primitive%20Component%20Object%20Reference) (OtherBodyIndex :type Integer) (bFromSweep :type Boolean) (SweepResult :type Hit%20Result%20Structure%20%28by%20ref%29))
  (Class|Projectail|DamageAfterOverlap OverlappedComponent OtherActor OtherComp OtherBodyIndex bFromSweep SweepResult true))

(event OnComponentHit(ProjectailMesh)
  (params (HitComponent :type Primitive%20Component%20Object%20Reference) (OtherActor :type Actor%20Object%20Reference) (OtherComp :type Primitive%20Component%20Object%20Reference) (NormalImpulse :type Vector :default "0, 0, 0") (Hit :type Hit%20Result%20Structure%20%28by%20ref%29))
  (Class|DamageIntarface|DoDamage(Message) OtherActor (Variables|Default|GetProjectailDamage) 0 self "VE_Bullet")
  (Class|Projectail|DestroyProjectailItself (.Location (Collision|BreakHitResult Hit))))

(fn ConstructionScript
  (bind _returnvalue (Rendering|Material|CreateDynamicMaterialInstance (Variables|Default|GetProjectailMesh) 0 "/Game/Game/Materials/M_SimpleUnlit.M_SimpleUnlit" :!class /Script/Engine.PrimitiveComponent))
  (Rendering|Material|SetVectorParameterValue _returnvalue "Color" (Variables|Default|GetColor) :!class /Script/Engine.MaterialInstanceDynamic))