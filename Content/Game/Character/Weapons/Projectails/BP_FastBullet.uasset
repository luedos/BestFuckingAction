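; BP_FastBullet is a weapon projectile that deals Bullet-type damage to what it hits.
; Mesh overlaps are forwarded to DamageAfterOverlap.
; The Hit event sends a damage message to the other actor, quarters the RGB of ProjectailColor while keeping alpha, then destroys the projectile at the hit location.
; The construction script creates a dynamic material on the mesh and tints it with ProjColor.
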(event OnComponentBeginOverlap(ProjectailMesh)
  (params (OverlappedComponent :type Primitive%20Component%20Object%20Reference) (OtherActor :type Actor%20Object%20Reference) (OtherComp :type Primitive%20Component%20Object%20Reference) (OtherBodyIndex :type Integer) (bFromSweep :type Boolean) (SweepResult :type Hit%20Result%20Structure%20%28by%20ref%29))
  (Class|Projectail|DamageAfterOverlap OverlappedComponent OtherActor OtherComp OtherBodyIndex bFromSweep SweepResult true))

(event Collision|EventHit
  (params (MyComp :type Primitive%20Component%20Object%20Reference) (Other :type Actor%20Object%20Reference) (OtherComp :type Primitive%20Component%20Object%20Reference) (bSelfMoved :type Boolean) (HitLocation :type Vector) (HitNormal :type Vector) (NormalImpulse :type Vector :default "0, 0, 0") (Hit :type Hit%20Result%20Structure%20%28by%20ref%29))
  (bind _returnvalue (Math|Byte|MakeLiteralByte 4))
  (Class|DamageIntarface|DoDamage(Message) Other (Variables|Default|GetProjectailDamage) 0 self "VE_Bullet")
  (bind _output_get (Variables|Default|SetProjectailColor (Math|Color|MakeColor (/ (.B (Math|Color|BreakColor (stale _output_get))) _returnvalue) (/ (.G (Math|Color|BreakColor (stale _output_get))) _returnvalue) (/ (.R (Math|Color|BreakColor (stale _output_get))) _returnvalue) (.A (Math|Color|BreakColor (stale _output_get))))))
  (Class|Projectail|DestroyProjectailItself HitLocation))

(fn ConstructionScript
  (bind _projectailmesh (Variables|Default|GetProjectailMesh))
  (bind _returnvalue (Rendering|Material|CreateDynamicMaterialInstance _projectailmesh 0 (Rendering|Material|GetMaterial _projectailmesh 0) :!class /Script/Engine.PrimitiveComponent))
  (bind _output_get (Variables|Default|SetMat _returnvalue))
  (Rendering|Material|SetVectorParameterValue _output_get "Color" (Variables|Default|GetProjColor) :!class /Script/Engine.MaterialInstanceDynamic))