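; BP_TurretBullet is a projectile Blueprint for a turret bullet that deals damage and removes itself on contact.
; An overlap on the projectile mesh passes to DamageAfterOverlap with destruction afterward, while a hit destroys the projectile at its current location.
; The construction script creates a dynamic material on the mesh and tints it with a brightened Color variable.
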(event OnComponentBeginOverlap(ProjectailMesh)
  (params (OverlappedComponent :type Primitive%20Component%20Object%20Reference) (OtherActor :type Actor%20Object%20Reference) (OtherComp :type Primitive%20Component%20Object%20Reference) (OtherBodyIndex :type Integer) (bFromSweep :type Boolean) (SweepResult :type Hit%20Result%20Structure%20%28by%20ref%29))
  (Class|Projectail|DamageAfterOverlap OtherActor OtherComp SweepResult true))

(event Collision|EventHit
  (params (MyComp :type Primitive%20Component%20Object%20Reference) (Other :type Actor%20Object%20Reference) (OtherComp :type Primitive%20Component%20Object%20Reference) (bSelfMoved :type Boolean) (HitLocation :type Vector :default "0, 0, 0") (HitNormal :type Vector :default "0, 0, 0") (NormalImpulse :type Vector :default "0, 0, 0") (Hit :type Hit%20Result%20Structure%20%28by%20ref%29))
  (Class|Projectail|DestroyProjectailItself (Transformation|GetActorLocation)))

(fn ConstructionScript
  (bind _projectailmesh (Variables|Default|GetProjectailMesh))
  (bind _returnvalue (Rendering|Material|CreateDynamicMaterialInstance _projectailmesh 0 (Rendering|Material|GetMaterial _projectailmesh 0) :!class /Script/Engine.PrimitiveComponent))
  (Rendering|Material|SetVectorParameterValue _returnvalue "Color" (* (Variables|Default|GetColor) 4.0) :!class /Script/Engine.MaterialInstanceDynamic))