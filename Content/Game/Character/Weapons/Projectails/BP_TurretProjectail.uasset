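; BP_TurretProjectail is a projectile that bursts into a ring of eight BP_TurretBullet actors on a hit or damaging overlap.
; Expload spaces the bullets evenly in yaw around the velocity heading, passes on team settings, then destroys the projectile.
; The construction script applies scale and tints the mesh through a dynamic material.
; A hit-count limit exists but is disconnected, so any Hit event explodes immediately.
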(event OnComponentBeginOverlap(ProjectailMesh)
  (params (OverlappedComponent :type Primitive%20Component%20Object%20Reference) (OtherActor :type Actor%20Object%20Reference) (OtherComp :type Primitive%20Component%20Object%20Reference) (OtherBodyIndex :type Integer) (bFromSweep :type Boolean) (SweepResult :type Hit%20Result%20Structure%20%28by%20ref%29))
  (bind _returnvalue (Class|Projectail|DamageAfterOverlap OtherActor OtherComp SweepResult true))
  (if _returnvalue
    (CallFunction|Expload)))

(event Custom|Expload
  (for _index (range 0 7)
    (Game|SpawnActorfromClass "/Game/Game/Character/Weapons/Projectails/BP_TurretBullet.BP_TurretBullet_C" (Math|Transform|MakeTransform (+ (Transformation|GetActorLocation) (* (Math|Rotator|GetRotationXVector (Math|Rotator|MakeRotator 0.0 0.0 (+ (.Yaw (Math|Rotator|BreakRotator (Math|Conversions|RotationFromXVector (Variables|/Script/Engine.MovementComponent|GetVelocity (Variables|Default|GetProjectileMovement))))) (* _index 45.0)))) 2e+01)) (Math|Rotator|MakeRotator 0.0 0.0 (+ (.Yaw (Math|Rotator|BreakRotator (Math|Conversions|RotationFromXVector (Variables|/Script/Engine.MovementComponent|GetVelocity (Variables|Default|GetProjectileMovement))))) (* _index 45.0))) "1,1,1") "Undefined" 0 0 (Variables|Default|GetProjectailTeam) (Variables|Default|GetbUseTeamVariable)))
  (Class|Projectail|DestroyProjectailItself (Transformation|GetActorLocation)))

(event EventBeginPlay)

(event Collision|EventActorBeginOverlap
  (params (OtherActor :type Actor%20Object%20Reference)))

(event EventTick
  (params (DeltaSeconds :type Float%20%28single-precision%29)))

(event Collision|EventHit
  (params (MyComp :type Primitive%20Component%20Object%20Reference) (Other :type Actor%20Object%20Reference) (OtherComp :type Primitive%20Component%20Object%20Reference) (bSelfMoved :type Boolean) (HitLocation :type Vector :default "0, 0, 0") (HitNormal :type Vector) (NormalImpulse :type Vector :default "0, 0, 0") (Hit :type Hit%20Result%20Structure%20%28by%20ref%29))
  (CallFunction|Expload))

(fn ConstructionScript
  (bind _projectailmesh (Variables|Default|GetProjectailMesh))
  (Transformation|SetWorldScale3D _projectailmesh (Variables|Default|GetScale))
  (bind _returnvalue (Rendering|Material|CreateDynamicMaterialInstance (Variables|Default|GetProjectailMesh) 0 (Rendering|Material|GetMaterial _projectailmesh 0) :!class /Script/Engine.PrimitiveComponent))
  (Rendering|Material|SetVectorParameterValue _returnvalue "Color" (Variables|Default|GetColor) :!class /Script/Engine.MaterialInstanceDynamic))