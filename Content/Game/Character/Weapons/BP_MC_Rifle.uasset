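; Rifle weapon Blueprint that adds colored trail particle effects when it is created.
; On the creation event, it gets its SMC and, if valid, loops through that object's components array, spawning an attached trail emitter on each component without auto-destroy.
; Each emitter is stored in a particle array and given a dynamic material instance with its Color parameter tinted dark gold.
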(event EventOnCreatedBNE
  (bind _returnvalue (Class|MCWeapon|GetSMC))
  (Utilities|IsValid _returnvalue
    (:Is%20Valid
      (bind _returnvalue_2 (Class|WeaponSMC|GetComponentsArray _returnvalue))
      (for _array_element _returnvalue_2
        (bind _returnvalue_3 (Effects|SpawnEmitterAttached (Variables|Default|GetTrailParticle) _array_element "None" (.location (Transformation|GetWorldTransform _array_element)) (.rotation (Transformation|GetWorldTransform _array_element)) "KeepRelativeOffset" false))
        (Utilities|Array|Add (Variables|Default|GetParticlesArray) _returnvalue_3)
        (bind _returnvalue_4 (Rendering|Material|CreateDynamicMaterialInstance _returnvalue_3 0 (Rendering|Material|GetMaterial _returnvalue_3 0) :!class /Script/Engine.PrimitiveComponent))
        (Rendering|Material|SetVectorParameterValue _returnvalue_4 "Color" "(R=0.510000,G=0.382500,B=0.000000,A=1.000000)" :!class /Script/Engine.MaterialInstanceDynamic)))))