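; BP_MC_LaserBeam is a weapon Blueprint that draws colored particle trails on the components supplied by its SMC.
; On creation it attaches a trail emitter to each component, begins trails between two sockets and tints a dynamic material magenta.
; Start and end events toggle trails on the stored emitters, with a debug print on start.
; Despite the name, the beam-fire setup is disconnected and never runs.
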(event EventOnCreatedBNE
  (bind _returnvalue (Class|MCWeapon|GetSMC))
  (Utilities|IsValid _returnvalue
    (:Is%20Valid
      (bind _returnvalue_2 (Class|WeaponSMC|GetComponentsArray _returnvalue))
      (for _array_element _returnvalue_2
        (bind _returnvalue_3 (Effects|SpawnEmitterAttached (Variables|Default|GetTrailParticle) _array_element "None" (.location (Transformation|GetWorldTransform _array_element)) (.rotation (Transformation|GetWorldTransform _array_element)) "KeepRelativeOffset" false))
        (Utilities|Array|Add (Variables|Default|GetParticlesArray) _returnvalue_3)
        (Effects|Particles|Trails|BeginTrails _returnvalue_3 "TrailSocket1" "TrailSocket2" "ETrailWidthMode_FromCentre" 1.0)
        (bind _returnvalue_4 (Rendering|Material|CreateDynamicMaterialInstance _returnvalue_3 0 (Rendering|Material|GetMaterial _returnvalue_3 0) :!class /Script/Engine.PrimitiveComponent))
        (Rendering|Material|SetVectorParameterValue _returnvalue_4 "Color" "(R=0.415000,G=0.041624,B=0.304135,A=1.000000)" :!class /Script/Engine.MaterialInstanceDynamic)))))

(event EventStartTrailBNE
  (for _array_element (Variables|Default|GetParticlesArray)
    (Development|PrintString (Class|MCWeapon|GetChar) (Utilities|GetDisplayName _array_element))
    (Effects|Particles|Trails|BeginTrails _array_element "TrailSocket1" "TrailSocket2" "ETrailWidthMode_FromCentre" 1.0)))

(event EventEndTrailBNE
  (for _array_element (Variables|Default|GetParticlesArray)
    (Effects|Particles|Trails|EndTrails _array_element)))