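; Enemy character Bolvan that fires bullet bursts at a visible target and handles its own death.
; A Delay-throttled Tick reads the AI blackboard state and enemy, checks visibility, then calls EnemyFire for timed, yaw-scattered shots, optionally rechecking sight per shot.
; Death plays tinted particles and sound, notifies the first BP_BotDeathRegistr, then destroys the actor a frame later.
; The construction script sockets the static mesh and colors its dynamic material.
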(event EventDeathStatus
  (bind _returnvalue (Effects|SpawnEmitteratLocation "/Game/Game/Particles/Char/P_BotDead.P_BotDead" (Transformation|GetActorLocation)))
  (Effects|Components|ParticleSystem|SetColorParameter _returnvalue "ParticleColor" "(R=0.030834,G=0.625342,B=0.885000,A=1.000000)")
  (Audio|PlaySoundatLocation "/Game/Game/Sounds/Death/S_BotDeath.S_BotDeath" (Transformation|GetActorLocation))
  (bind _outactors (Actor|GetAllActorsOfClass "/Game/Game/Levels/BP_BotDeathRegistr.BP_BotDeathRegistr_C"))
  (if (!= (Utilities|Array|Length _outactors) 0)
    (Default|CallCallforDeath (Utilities|Array|Get(acopy) _outactors) (Transformation|GetActorLocation) (Utilities|GetClass self) self))
  (Class|LowEntryExtendedStandardLibrary|DelayFrames 1)
  (Actor|DestroyActor))

(event EventEnemyFire
  (params (NumberOfFire :type Integer) (Target :type Actor%20Object%20Reference) (ShootWhileVisible :type Boolean))
  (bind _returnvalue (Transformation|GetActorLocation))
  (bind _returnvalue_2 (Transformation|GetActorLocation Target))
  (bind _returnvalue_3 (Math|Random|RandomFloatinRange -7.0 7.0))
  (bind _self self)
  (bind _returnvalue_4 (Math|Rotator|FindLookatRotation _returnvalue _returnvalue_2))
  (bind _returnvalue_5 (+ (.yaw _returnvalue_4) _returnvalue_3))
  (Variables|Default|SetNumOfShots 0)
  (Utilities|IsValid Target
    (:Is%20Valid
      (if ShootWhileVisible :!label _label
        (bind _returnvalue_6 (Class|CharPawn|TestforVisibilityonActor Target))
        (if _returnvalue_6
          (if (< (Variables|Default|GetNumOfShots) NumberOfFire) :!label _label_2
            (Game|SpawnActorfromClass "/Game/Game/Character/Weapons/Projectails/BP_BolvanBullet.BP_BolvanBullet_C" (Math|Transform|MakeTransform (+ _returnvalue (* (Math|Rotator|GetRotationXVector (Math|Rotator|MakeRotator 0.0 (.pitch _returnvalue_4) _returnvalue_5)) 1e+02)) (Math|Rotator|MakeRotator 0.0 (.pitch _returnvalue_4) _returnvalue_5) "1,1,1") "Undefined" _self _self "TE_Enemy" true)
            (Audio|SpawnSoundatLocation "/Game/Game/Sounds/BolvanBullet/S_BolvanBullet_Fire.S_BolvanBullet_Fire" (Transformation|GetActorLocation))
            (bind _output_get (Variables|Default|SetNumOfShots (+ (stale _output_get) 1)))
            (Utilities|FlowControl|Delay 0.2)
            (goto _label)))
        (else
          (goto _label_2))))))

(event EventDoDamage
  (params (Damage :type Float%20%28single-precision%29) (DamageFromTeam :type ETeamEnum%20Enum :default "TE_Player") (Couser :type Actor%20Object%20Reference) (DamageType :type EDamageType%20Enum :default "VE_Bullet"))
  (Class|CharPawn|DamageHP Damage))

(event EventTick
  (params (DeltaSeconds :type Float%20%28single-precision%29))
  (Utilities|FlowControl|Delay 1.5)
  (bind _returnvalue (AI|GetAIController self))
  (if (> (Class|BlackboardComponent|GetValueasEnum (AI|GetBlackboard _returnvalue) (Utilities|Name|MakeLiteralName "EnumKey")) 1)
    (bind _ascharacter (Utilities|Casting|CastToCharacter (AI|Components|Blackboard|GetValueasObject (AI|GetBlackboard _returnvalue) (Utilities|Name|MakeLiteralName "Enemy"))))
    (bind _returnvalue_2 (Class|CharPawn|TestforVisibilityonActor _ascharacter))
    (if _returnvalue_2
      (Class|EnemyChar|EnemyFire 3 _ascharacter false))))

(fn ConstructionScript
  (bind _staticmesh (Variables|Default|GetStaticMesh))
  (Transformation|AttachComponentToComponent (Variables|Default|GetStaticMesh) (Variables|Character|GetMesh) "MeshSocket" "SnapToTarget" "SnapToTarget" "KeepRelative" true)
  (bind _returnvalue (Rendering|Material|CreateDynamicMaterialInstance _staticmesh 0 (Rendering|Material|GetMaterial _staticmesh 0) :!class /Script/Engine.PrimitiveComponent))
  (Rendering|Material|SetVectorParameterValue _returnvalue "Color" (Variables|Default|GetColor) :!class /Script/Engine.MaterialInstanceDynamic))