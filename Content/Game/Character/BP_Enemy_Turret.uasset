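; BP_Enemy_Turret is a turret enemy that opens and closes, fires projectiles and takes damage only while open.
; SetOpen scales the dynamic material's color brighter or dimmer and passes the state to the AB_Turret animation Blueprint.
; EnemyFire spawns an enemy-team projectile ahead of the arrow component and triggers the fire animation.
; DeathStatus spawns a tinted death particle and destroys the actor.
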(event EventDoDamage
  (params (Damage :type Float%20%28single-precision%29) (CallInstigator :type Player%20Controller%20Object%20Reference) (Couser :type Actor%20Object%20Reference) (DamageType :type EDamageType%20Enum :default "VE_Bullet"))
  (if (Variables|Default|GetIsOpen)
    (Class|CharPawn|DamageHP Damage)
    (Development|PrintString (Utilities|String|ToString(Float) Damage))))

(event EventEnemyFire
  (params (NumberOfFire :type Integer) (Target :type Actor%20Object%20Reference) (ShootWhileVisible :type Boolean))
  (bind _self self)
  (bind _arrowcomponent (Variables|Default|GetArrowComponent))
  (bind _returnvalue (Transformation|GetWorldTransform _arrowcomponent))
  (Game|SpawnActorfromClass "/Game/Game/Character/Weapons/Projectails/BP_TurretProjectail.BP_TurretProjectail_C" (Math|Transform|MakeTransform (+ (.location _returnvalue) (* (Math|Rotator|GetRotationXVector (.rotation _returnvalue)) 4e+01)) (.rotation _returnvalue) "1,1,1") "Undefined" _self _self "TE_Enemy" true _self)
  (bind _asab_turret (Utilities|Casting|CastToAB_Turret (Components|SkeletalMesh|GetAnimInstance (Variables|Character|GetMesh))))
  (Variables|/Game/Game/Meshs/Turret/AB_Turret.AB_Turret_C|SetFire _asab_turret true))

(event EventDeathStatus
  (bind _returnvalue (Effects|SpawnEmitteratLocation "/Game/Game/Particles/Char/P_BotDead.P_BotDead" (Transformation|GetActorLocation)))
  (Effects|Components|ParticleSystem|SetColorParameter _returnvalue "ParticleColor" "(R=1.000000,G=0.000000,B=0.862993,A=1.000000)")
  (Actor|DestroyActor))

(event EventSetOpen
  (params (InState :type Boolean))
  (if (Math|Boolean|NotEqual(Boolean) InState (Variables|Default|GetIsOpen))
    (Variables|Default|SetIsOpen InState)
    (if InState
      (bind _output_get (Variables|Default|SetColor (* (stale _output_get) 4.0)))
      (else
        (bind _output_get_2 (Variables|Default|SetColor (* (stale _output_get_2) 0.25)))))
    (Rendering|Material|SetVectorParameterValue (Variables|Default|GetMeshMat) "Color" (Variables|Default|GetColor) :!class /Script/Engine.MaterialInstanceDynamic)
    (bind _asab_turret (Utilities|Casting|CastToAB_Turret (Components|SkeletalMesh|GetAnimInstance (Variables|Character|GetMesh))))
    (Variables|/Game/Game/Meshs/Turret/AB_Turret.AB_Turret_C|SetOpen _asab_turret (Variables|Default|GetIsOpen))))

(fn ConstructionScript
  (bind _mesh (Variables|Character|GetMesh))
  (bind _returnvalue (Rendering|Material|CreateDynamicMaterialInstance _mesh 0 (Rendering|Material|GetMaterial _mesh 0) :!class /Script/Engine.PrimitiveComponent))
  (bind _output_get (Variables|Default|SetMeshMat _returnvalue))
  (Rendering|Material|SetVectorParameterValue _output_get "Color" (Variables|Default|GetColor) :!class /Script/Engine.MaterialInstanceDynamic))