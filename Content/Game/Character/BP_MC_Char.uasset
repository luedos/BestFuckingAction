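; Player character Blueprint that implements effects for spin, dash, firing and reload events, plus HUD, options menu, camera rotation and death handling.
; Spin sphere-traces to trigger pickups; spin and fire flash a dynamic material color that a looping timer interpolates back to idle.
; Death hides the character, resets enemy AI blackboards and shows Game Over.
; Debug keys toggle energy gates and god mode; weapon construction and attachment code is disconnected.
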(event Custom|SetInterpColorFunc
  (params (InColor :type Linear%20Color%20Structure) (InColorInterpSpeed :type Float%20%28single-precision%29))
  ;[1 1 1] Some functions
  (Variables|Default|SetColorInterpSpeed InColorInterpSpeed)
  (Rendering|Material|SetVectorParameterValue (Variables|Default|GetMeshMat) "Color" InColor :!class /Script/Engine.MaterialInstanceDynamic)
  (Variables|Default|SetColor InColor)
  (Utilities|Time|SetTimerbyFunctionName 0 "InterpDeafoltColor" 0.03 true))

(event EventBeginPlay
  (Class|CharPawn|SetCanCharbeDamaged true)
  ;[1 1 1] Create Char hud
  (bind _returnvalue (UserInterface|CreateWidget "/Game/Game/HUD/UI_MCHUD.UI_MCHUD_C" (Game|GetPlayerController 0)))
  (bind _output_get (Variables|HUD|SetHud _returnvalue))
  (Variables|/Game/Game/HUD/UI_MCHUD.UI_MCHUD_C|SetChar _output_get self)
  (UserInterface|Viewport|AddtoViewport _output_get 0))

(event EventDoDamage
  (params (Damage :type Float%20%28single-precision%29) (DamageFromTeam :type ETeamEnum%20Enum :default "TE_Player") (Couser :type Actor%20Object%20Reference) (DamageType :type EDamageType%20Enum :default "VE_Bullet"))
  ;[1 1 1] For damage
  (Class|CharPawn|DamageHP Damage))

(event EventFireBNE
  (params (Weapon :type MC%20Weapon%20Object%20Reference) (IsPrimeFire :type Boolean) (FireOrMisfire :type Boolean))
  ;[1 1 1] Fire function
  (CallFunction|SetInterpColorFunc "(R=0.000000,G=3.000000,B=0.242048,A=1.000000)" 7.0)
  (Utilities|Casting|CastToMC_Rifle Weapon)
  (if IsPrimeFire
    (Audio|SpawnSoundatLocation 0 (Transformation|GetActorLocation))
    (Effects|SpawnEmitteratLocation (Class|MCWeapon|GetFireParticle Weapon IsPrimeFire) "0, 0, 0")))

(event EventTick
  (params (DeltaSeconds :type Float%20%28single-precision%29))
  (bind _returnvalue (Game|GetPlayerController 0))
  (bind _mousepos (Variables|Default|GetMousePos))
  ;[1 1 1] Camera Rotation Function
  (Utilities|FlowControl|Sequence
    (:then_0
      (if (Variables|Default|GetIsRotateCamera)
        (Transformation|AddWorldRotation (Variables|Default|GetCameraRotationArrow) (Math|Rotator|MakeRotator 0.0 0.0 (Class|Actor|GetInputAxisKeyValue)) false false)
        (Class|LowEntryExtendedStandardLibrary|SetMousePosition (Math|Float|Truncate (.x _mousepos)) (Math|Float|Truncate (.y _mousepos)))))
    (:then_1
      ;[1 1 1] Rotate actor mesh
      (Transformation|AddWorldRotation (Variables|Default|GetCharMesh) (Math|Rotator|MakeRotator 0.0 (* DeltaSeconds (Math|Trig|Sin(Radians) (Utilities|Time|GetGameTimeinSeconds)) 6e+01) (* DeltaSeconds 6e+01)) false false))
    (:then_2
      (if (and (not (Variables|/Script/Engine.PlayerController|GetbShowMouseCursor _returnvalue)) (Variables|Default|GetAllwaysShowCursor))
        (Variables|/Script/Engine.PlayerController|SetbShowMouseCursor _returnvalue true)))))

(event EventStopReloadingBNE
  (bind _reloadparticle (Variables|Default|GetReloadParticle))
  ;[1 1 1] Reload functions
  (Utilities|IsValid _reloadparticle
    (:Is%20Valid
      (Components|DestroyComponent _reloadparticle))))

(event EventChangeWeaponBNE
  ;[1 1 1] Changing weapon (not using for now)
)

(event EventStartReloadBNE
  (bind _returnvalue (Class|MCChar|GetIsFirstWeapon))
  (bind _firstweapon (Variables|Default|GetFirstWeapon))
  (bind _secondweapon (Variables|Default|GetSecondWeapon))
  (bind _returnvalue_2 (select _returnvalue _firstweapon _secondweapon))
  ;[1 1 1] Reload functions
  (Utilities|IsValid (Variables|Default|GetReloadParticle)
    (:Is%20Valid
      (Components|DestroyComponent (Variables|Default|GetReloadParticle)))
    (:Is%20Not%20Valid
      _))
  (bind _returnvalue_3 (Effects|SpawnEmitterAttached (Class|MCWeapon|GetReloadParticle _returnvalue_2) (Variables|Default|GetCapsuleComponent) "None" "0, 0, 0" "0, 0, 0" "SnapToTarget"))
  (bind _output_get (Variables|Default|SetReloadParticle _returnvalue_3))
  (Effects|Components|ParticleSystem|SetFloatParameter _output_get "ParticleLifeTime" (Class|MCWeapon|GetReloadRate _returnvalue_2)))

(event EventSpiningEventImplementation
  (bind _returnvalue (Transformation|GetActorLocation))
  (bind _capsulecomponent (Variables|Default|GetCapsuleComponent))
  ;[1 1 1] Spining function
  (bind _outhits (Collision|MultiSphereTraceForObjects _returnvalue (+ _returnvalue "0, 0,1.000000") (Variables|Default|GetSpiningRadius) (Utilities|Array|MakeArray "ObjectTypeQuery8") false 0 "None"))
  (for _array_element _outhits
    (if (Utilities|DoesObjectImplementInterface (.HitActor (Collision|BreakHitResult _array_element)) "/Script/Demo_001.PickUpInterface")
      (Class|PickUpInterface|PickUpFunc(Message) (.HitActor (Collision|BreakHitResult _array_element)) self)))
  (Effects|SpawnEmitterAttached "/Game/Game/Particles/Char/P_Spining.P_Spining" _capsulecomponent "None" "0, 0, 0" (Transformation|GetWorldRotation _capsulecomponent) "SnapToTarget")
  (CallFunction|SetInterpColorFunc "(R=0.000000,G=0.277805,B=5.000000,A=1.000000)" 2.0)
  (Audio|SpawnSoundAttached "/Game/Game/Sounds/Spining/S_Spining.S_Spining" (Variables|Default|GetCharMesh)))

(event EventDeshEventImplementation
  (params (DeshDirection :type Vector))
  (bind _trailparticle (Variables|Default|GetTrailParticle))
  ;[1 1 1] Desh
  (Audio|SpawnSoundAttached "/Game/Game/Sounds/Desh/S_Desh.S_Desh" (Variables|Default|GetCharMesh))
  (if (Variables|Desh|GetShowDeshTrail)
    (Transformation|SetWorldRotation (Variables|Default|GetTrailMesh) (Math|Rotator|MakeRotator 0.0 0.0 (.yaw (Math|Conversions|RotationFromXVector DeshDirection))) false false)
    (Effects|Particles|Trails|BeginTrails _trailparticle "TrailSocket1" "TrailSocket2" "ETrailWidthMode_FromCentre" 1.0)
    (Utilities|FlowControl|Delay 0.3)
    (Effects|Particles|Trails|EndTrails _trailparticle)))

(event EventDeathStatus
  (bind _returnvalue (Game|GetPlayerController 0))
  (bind _returnvalue_2 (Transformation|GetActorTransform))
  ;[1 1 1] For damage
  (Class|CharPawn|SetCanCharbeDamaged false)
  (Utilities|IsValid (Variables|HUD|GetGameOverScreen)
    (:Is%20Valid
      (if (not (UserInterface|Viewport|IsinViewport (Variables|HUD|GetGameOverScreen)))
        (Viewport|RemoveAllWidgets :!label _label)
        (Variables|Default|SetbCanMove false)
        (Input|DisableInput _returnvalue)
        (AI|Navigation|StopMovement _returnvalue)
        (bind _outactors (Actor|GetAllActorsOfClass "/Script/Demo_001.AIC_Enemy"))
        (for _array_element _outactors
          (AI|Components|Blackboard|SetValueasEnum (AI|GetBlackboard _array_element) (Utilities|Name|MakeLiteralName "EnumKey")))
        (bind _returnvalue_3 (Effects|SpawnEmitteratLocation "/Game/Game/Particles/Char/P_BotDead.P_BotDead" (.location _returnvalue_2) (.rotation _returnvalue_2)))
        (Effects|Components|ParticleSystem|SetColorParameter _returnvalue_3 "ParticleColor" "(R=0.050000,G=0.050000,B=1.000000,A=1.000000)")
        (Effects|Components|ParticleSystem|SetFloatParameter _returnvalue_3 "Count" 1.5)
        (Rendering|SetActorHiddenInGame true)
        (Utilities|FlowControl|Delay 0.5)
        (bind _returnvalue_4 (UserInterface|CreateWidget "/Game/Game/HUD/GO_Screen.GO_Screen_C"))
        (Variables|HUD|SetGameOverScreen _returnvalue_4)
        (UserInterface|Viewport|AddtoViewport _returnvalue_4 0)
        (Variables|/Script/Engine.PlayerController|SetbShowMouseCursor (Game|GetPlayerController 0) true)))
    (:Is%20Not%20Valid
      (goto _label))))

(event Input|ActionEvents|InputActionRotateCamera
  (params (Key :type Key%20Structure :default "AnyKey"))
  (bind _returnvalue (Game|GetPlayerController 0))
  ;[1 1 1] Camera Rotation Function
  (:Pressed
    (Variables|Default|SetIsRotateCamera true)
    (Variables|/Script/Engine.PlayerController|SetbShowMouseCursor _returnvalue false)
    (bind (_success _x _y) (Class|LowEntryExtendedStandardLibrary|GetMousePosition))
    (Variables|Default|SetMousePos (Math|Vector2D|MakeVector2D (Math|Conversions|ToFloat(Integer) _x) (Math|Conversions|ToFloat(Integer) _y))))
  (:Released
    (Variables|Default|SetIsRotateCamera false)
    (Variables|/Script/Engine.PlayerController|SetbShowMouseCursor _returnvalue false)))

(event Input|KeyboardEvents|F
  (params (Key :type Key%20Structure :default "AnyKey"))
  (bind _returnvalue (Game|GetPlayerController 0))
  ;[1 1 1] Options Menu
  (:Pressed
    (if (Utilities|IsValid (Variables|HUD|GetOptions))
      (if (UserInterface|Viewport|IsinViewport (Variables|HUD|GetOptions))
        (Widget|RemovefromParent (Variables|HUD|GetOptions))
        (Input|SetInputModeGameOnly (Game|GetPlayerController 0))
        (Variables|/Script/Engine.PlayerController|SetbShowMouseCursor _returnvalue false)
        (else
          (Variables|/Script/Engine.PlayerController|SetbShowMouseCursor _returnvalue true :!label _label)
          (bind _returnvalue_2 (UserInterface|CreateWidget "/Game/Game/HUD/UI_Options.UI_Options_C" _returnvalue))
          (Variables|HUD|SetOptions _returnvalue_2)
          (Variables|/Game/Game/HUD/UI_Options.UI_Options_C|SetChar _returnvalue_2 self)
          (UserInterface|Viewport|AddtoViewport _returnvalue_2 0)
          (Input|SetInputModeGameandUI (Game|GetPlayerController 0) _returnvalue_2 "LockAlways" false)))
      (else
        (goto _label)))))

(event Input|KeyboardEvents|G
  (params (Key :type Key%20Structure :default "AnyKey"))
  (bind _bcancharbedamaged (Variables|Default|GetbCanCharBeDamaged))
  ;[1 1 1] Some functions
  (:Pressed
    (Class|CharPawn|SetCanCharbeDamaged (not _bcancharbedamaged))
    (Development|PrintString (Utilities|String|Append "God mod : " (select _bcancharbedamaged "Off" "On")))))

(event Input|KeyboardEvents|V
  (params (Key :type Key%20Structure :default "AnyKey"))
  ;[1 1 1] Some functions
  (:Pressed
    (bind _output_get (Variables|Default|SetSpiningStatus (+ (stale _output_get) 1)))
    (if (> _output_get 2)
      (Variables|Default|SetSpiningStatus 0))
    (Development|PrintString (Utilities|String|Append "Spining Status: " (Utilities|String|ToString(Integer) (Variables|Default|GetSpiningStatus))))))

(event Input|KeyboardEvents|T
  (params (Key :type Key%20Structure :default "AnyKey"))
  (:Pressed
    (bind _outactors (Actor|GetAllActorsOfClass "/Game/Game/Levels/LevelsProps/BP_EnergyGate.BP_EnergyGate_C"))
    (Utilities|FlowControl|FlipFlop
      (:A
        (Default|OpenElGate _outactors))
      (:B
        (Default|CloseElGate _outactors)))))

(fn ConstructionScript
  (bind _charmesh (Variables|Default|GetCharMesh))
  (Transformation|AttachComponentToComponent (Variables|Default|GetCharMesh) (Variables|Character|GetMesh) "ActiveGunSocket" "SnapToTarget" "SnapToTarget" "SnapToTarget" true)
  (bind _returnvalue (Rendering|Material|CreateDynamicMaterialInstance _charmesh 0 (Rendering|Material|GetMaterial _charmesh 0) :!class /Script/Engine.PrimitiveComponent))
  (bind _output_get (Variables|Default|SetMeshMat _returnvalue))
  (Rendering|Material|SetVectorParameterValue _output_get "Color" (Variables|Default|GetIdleColor) :!class /Script/Engine.MaterialInstanceDynamic))

(fn InterpDeafoltColor
  (Rendering|Material|SetVectorParameterValue (Variables|Default|GetMeshMat) "Color" (Class|KismetMathLibrary|CInterpto (Variables|Default|GetColor) (Variables|Default|GetIdleColor) 0.03 (Variables|Default|GetColorInterpSpeed)) :!class /Script/Engine.MaterialInstanceDynamic)
  (Variables|Default|SetColor (Class|KismetMathLibrary|CInterpto (Variables|Default|GetColor) (Variables|Default|GetIdleColor) 0.03 (Variables|Default|GetColorInterpSpeed)))
  (if (Math|Float|NearlyEqual(Float) (Math|Vector|VectorLength (- (Math|Conversions|ToVector(LinearColor) (Class|KismetMathLibrary|CInterpto (Variables|Default|GetColor) (Variables|Default|GetIdleColor) 0.03 (Variables|Default|GetColorInterpSpeed))) (Math|Conversions|ToVector(LinearColor) (Variables|Default|GetIdleColor)))) 0.0 0.001)
    (Utilities|Time|ClearTimerbyFunctionName 0 "InterpDeafoltColor")))