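; BP_Enemy_WIcoSphere is an enemy that fires spreads of small balls at a target, uses a shield, and has a crit component.
; EnemyFire calls OnDownBNE on the shield, then spawns three Enemy-team BP_SmallBall projectiles fanned in yaw, using a delayed loop to repeat.
; Construction socket-attaches the static mesh, selects BP_Shield, and tints body and crit component through dynamic materials.
; Damage feeds DamageHP; death spawns a colored particle burst and destroys the actor.
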(event EventDeathStatus
  (bind _returnvalue (Effects|SpawnEmitteratLocation "/Game/Game/Particles/Char/P_BotDead.P_BotDead" (Transformation|GetActorLocation)))
  (Effects|Components|ParticleSystem|SetColorParameter _returnvalue "ParticleColor" "(R=0.824234,G=0.000000,B=0.885000,A=1.000000)")
  (Actor|DestroyActor))

(event EventEnemyFire
  (params (NumberOfFire :type Integer) (Target :type Actor%20Object%20Reference) (ShootWhileVisible :type Boolean))
  (bind _returnvalue (Transformation|GetActorLocation))
  (bind _returnvalue_2 (Transformation|GetActorLocation Target))
  (bind _shieldcomponent (Variables|Default|GetShieldComponent))
  (bind _returnvalue_3 (Math|Rotator|FindLookatRotation _returnvalue _returnvalue_2))
  (Utilities|IsValid Target
    (:Is%20Valid
      (Utilities|FlowControl|Sequence
        (:then_0
          (if (!= _shieldcomponent 0)
            (if (Utilities|IsValid _shieldcomponent)
              (Class|Shield|OnDownBNE _shieldcomponent))))
        (:then_1
          (Variables|Default|SetNumOfShots 0)
          (for _index (range 0 2) :!label _label
            (Game|SpawnActorfromClass "/Game/Game/Character/Weapons/Projectails/BP_SmallBall.BP_SmallBall_C" (Math|Transform|MakeTransform (+ _returnvalue (* (Math|Rotator|GetRotationXVector (Math|Rotator|MakeRotator 0.0 (.pitch _returnvalue_3) (+ (.yaw _returnvalue_3) (* (/ (Variables|Default|GetSpread) 2.0) (Math|Conversions|ToFloat(Integer) (- _index 1)))))) 1e+02)) (Math|Rotator|MakeRotator 0.0 (.pitch _returnvalue_3) (+ (.yaw _returnvalue_3) (* (/ (Variables|Default|GetSpread) 2.0) (Math|Conversions|ToFloat(Integer) (- _index 1))))) "1,1,1") "Undefined" self 0 "TE_Enemy" true)
            (Variables|Default|SetNumOfShots (+ (Variables|Default|GetNumOfShots) 1))
            (Utilities|FlowControl|Delay 1.5)
            (if (< (Variables|Default|GetNumOfShots) NumberOfFire)
              (goto _label))))))))

(event EventDoDamage
  (params (Damage :type Float%20%28single-precision%29) (CallInstigator :type Player%20Controller%20Object%20Reference) (Couser :type Actor%20Object%20Reference) (DamageType :type EDamageType%20Enum :default "VE_Bullet"))
  (Development|PrintString (Utilities|String|ToString(Float) Damage))
  (Class|CharPawn|DamageHP Damage))

(fn ConstructionScript
  (bind _staticmesh (Variables|Default|GetStaticMesh))
  (bind _bp_kritcomponent (Variables|Default|GetBP_KritComponent))
  (Transformation|AttachComponentToComponent (Variables|Default|GetStaticMesh) (Variables|Character|GetMesh) "MeshSocket" "SnapToTarget" "SnapToTarget" "KeepRelative" true)
  (bind _returnvalue (Rendering|Material|CreateDynamicMaterialInstance _staticmesh 0 (Rendering|Material|GetMaterial _staticmesh 0) :!class /Script/Engine.PrimitiveComponent))
  (Rendering|Material|SetVectorParameterValue _returnvalue "Color" (Variables|Default|GetColor) :!class /Script/Engine.MaterialInstanceDynamic)
  (Variables|Default|SetUsingShield "/Game/Game/Components/BP_Shield.BP_Shield_C")
  (Class|KritComponent|OnCreatedKC _bp_kritcomponent self)
  (bind _returnvalue_2 (Rendering|Material|CreateDynamicMaterialInstance _bp_kritcomponent 0 (Rendering|Material|GetMaterial _bp_kritcomponent 0) :!class /Script/Engine.PrimitiveComponent))
  (Rendering|Material|SetVectorParameterValue _returnvalue_2 "Color" (Variables|Default|GetKritComponentColor) :!class /Script/Engine.MaterialInstanceDynamic))