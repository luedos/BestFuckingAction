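; Tetrahedron enemy character that shows dash trails, fires energy balls at targets and bursts into particles on death.
; Dash start and stop events toggle blue particle trails and a gated Tick that yaws the trail mesh toward the dash point.
; Firing waits a random short delay, then spawns an enemy-team projectile aimed at the target.
; Construction attaches and tints the body mesh, and damage is forwarded to DamageHP.
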(event EventStartDeshBNE
  (params (PointDeshRef :type Vector))
  (bind _particlesystem (Variables|Default|GetParticleSystem))
  (bind _trailstmesh (Variables|Default|GetTrailStMesh))
  (bind _particlesystem_2 (Variables|Default|GetParticleSystem))
  (bind _returnvalue (Rendering|Material|CreateDynamicMaterialInstance _particlesystem 0 (Rendering|Material|GetMaterial _particlesystem 0) :!class /Script/Engine.PrimitiveComponent))
  (Rendering|Material|SetVectorParameterValue _returnvalue "Color" "(R=0.080000,G=0.080000,B=1.000000,A=1.000000)" :!class /Script/Engine.MaterialInstanceDynamic)
  (Utilities|FlowControl|Sequence
    (:then_0
      (bind _output_get (Variables|Default|SetPointToDesh PointDeshRef))
      (Effects|Particles|Trails|BeginTrails _particlesystem_2 "TrailSocket1" "TrailSocket2" "ETrailWidthMode_FromCentre" 1.0)
      (Utilities|FlowControl|Delay 0.3)
      (Utilities|FlowControl|Sequence
        (:then_0
          (Utilities|FlowControl|Gate true :!label _label
            (:Exit
              (Utilities|FlowControl|Delay 0.1)
              (Effects|Particles|Trails|EndTrails _particlesystem_2)
              (Utilities|FlowControl|Gate true) ; enters at Close
            )))
        (:then_1
          (goto _label Open))))
    (:then_1
      (Utilities|FlowControl|Gate true) ; enters at Open
    )))

(event EventTick
  (params (DeltaSeconds :type Float%20%28single-precision%29))
  (bind _trailstmesh (Variables|Default|GetTrailStMesh))
  (Utilities|FlowControl|Gate true
    (:Exit
      (Transformation|SetWorldRotation _trailstmesh (Math|Rotator|MakeRotator 0.0 0.0 (.yaw (Math|Rotator|FindLookatRotation (Transformation|GetWorldLocation _trailstmesh) (stale EventStartDeshBNE _output_get)))) false false))))

(event EventStopDeshBNE
  (bind _trailstmesh (Variables|Default|GetTrailStMesh))
  (bind _particlesystem (Variables|Default|GetParticleSystem))
  (Utilities|FlowControl|Delay 0.1)
  (Effects|Particles|Trails|EndTrails _particlesystem)
  (Utilities|FlowControl|Sequence
    (:then_0
      (Utilities|FlowControl|Gate true) ; enters at Close
    )
    (:then_1
      (Utilities|FlowControl|Gate true) ; enters at Close
    )))

(event EventEnemyFire
  (params (NumberOfFire :type Integer) (Target :type Actor%20Object%20Reference) (ShootWhileVisible :type Boolean))
  (bind _returnvalue (Transformation|GetActorLocation))
  (bind _returnvalue_2 (Transformation|GetActorLocation Target))
  (Utilities|FlowControl|Delay (Math|Random|RandomFloatinRange 0.0 0.5))
  (Utilities|IsValid Target
    (:Is%20Valid
      (Game|SpawnActorfromClass "/Game/Game/Character/Weapons/Projectails/BP_EnergyBall.BP_EnergyBall_C" (Math|Transform|MakeTransform (+ _returnvalue (* (Math|Rotator|GetRotationXVector (Math|Rotator|FindLookatRotation _returnvalue _returnvalue_2)) 1e+02)) "0.0,0.0,0.0" "1,1,1") "AdjustIfPossibleButAlwaysSpawn" self _returnvalue_2 self "TE_Enemy" true))))

(event EventDeathStatus
  (bind _returnvalue (Effects|SpawnEmitteratLocation "/Game/Game/Particles/Char/P_BotDead.P_BotDead" (Transformation|GetActorLocation)))
  (Effects|Components|ParticleSystem|SetFloatParameter _returnvalue "Count" 0.5)
  (Effects|Components|ParticleSystem|SetColorParameter _returnvalue "ParticleColor" "(R=0.885000,G=0.697947,B=0.037176,A=1.000000)")
  (Actor|DestroyActor))

(event EventDoDamage
  (params (Damage :type Float%20%28single-precision%29) (CallInstigator :type Player%20Controller%20Object%20Reference) (Couser :type Actor%20Object%20Reference) (DamageType :type EDamageType%20Enum :default "VE_Bullet"))
  (Class|CharPawn|DamageHP Damage))

(event EventBeginPlay
  (Components|Activation|Activate (Variables|Default|GetParticleSystem) false))

(fn ConstructionScript
  (bind _staticmesh (Variables|Default|GetStaticMesh))
  (Transformation|AttachComponentToComponent (Variables|Default|GetStaticMesh) (Variables|Character|GetMesh) "MeshSocket" "SnapToTarget" "SnapToTarget" "KeepRelative" true)
  (bind _returnvalue (Rendering|Material|CreateDynamicMaterialInstance _staticmesh 0 (Rendering|Material|GetMaterial _staticmesh 0) :!class /Script/Engine.PrimitiveComponent))
  (Rendering|Material|SetVectorParameterValue _returnvalue "Color" (Variables|Default|GetColor) :!class /Script/Engine.MaterialInstanceDynamic)
  (Transformation|AttachComponentToComponent (Variables|Default|GetTrailStMesh) (Variables|Default|GetCapsuleComponent) "None" "SnapToTarget" "KeepWorld" "KeepWorld" true))