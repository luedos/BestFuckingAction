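; AI controller for the Icosphere enemy that runs its behavior tree and steers the direction of the pawn's facing arrow.
; BeginPlay starts BT_Icosphere, then waits one frame before calling the parent BeginPlay.
; Each tick it reads the blackboard EnumKey: in one state the arrow interpolates toward the Enemy actor, otherwise toward the pawn's velocity direction.
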(event EventBeginPlay
  (AI|RunBehaviorTree "/Game/Game/AI/Icosphere/BT_Icosphere.BT_Icosphere")
  (Class|LowEntryExtendedStandardLibrary|DelayFrames 1)
  (|CallParentFunction))

(event EventTick
  (params (DeltaSeconds :type Float%20%28single-precision%29))
  (bind _returnvalue (AI|GetBlackboard 0))
  (bind _returnvalue_2 (Utilities|Name|MakeLiteralName "Enemy"))
  (bind _returnvalue_3 (AI|Components|Blackboard|GetValueasObject _returnvalue _returnvalue_2))
  (bind _asenemy_wico_sphere (Utilities|Casting|CastToEnemy_WIcoSphere (Pawn|GetControlledPawn)))
  (if (== (Class|BlackboardComponent|GetValueasEnum _returnvalue (Utilities|Name|MakeLiteralName "EnumKey")) 2)
    (Utilities|IsValid _returnvalue_3
      (:Is%20Valid
        (bind _asactor (Utilities|Casting|CastToActor _returnvalue_3))
        (Class|EnemyWIcoSphere|InterpFaceArrow _asenemy_wico_sphere DeltaSeconds (Transformation|GetActorLocation _asactor))))
    (else
      (Class|EnemyWIcoSphere|InterpFaceArrow _asenemy_wico_sphere DeltaSeconds (+ (Transformation|GetVelocity _asenemy_wico_sphere) (Transformation|GetActorLocation _asenemy_wico_sphere))))))

(fn ConstructionScript
  (|CallParentFunction))