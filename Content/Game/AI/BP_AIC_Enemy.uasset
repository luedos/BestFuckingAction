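; Enemy AI controller that turns perception updates into blackboard state.
; On BeginPlay it stores the pawn and its starting position as the duty location.
; Unless perception is overridden, it picks the first living MC_Char among updated actors.
; If sensed, it sets that character as enemy and switches sight radius to the lose radius; otherwise it records the target's current location, with each case setting a different state enum.
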(event OnPerceptionUpdated(PerceptionComp)
  (params (UpdatedActors :type Array%20of%20Actor%20Object%20References))
  (bind _returnvalue (AI|GetBlackboard 0))
  (bind _returnvalue_2 (Utilities|Name|MakeLiteralName "EnumKey"))
  (if (not (Variables|Default|GetOverridePerception))
    (Variables|Default|SetFindSomeOne false)
    (bind _array_element (Utilities|Array|ForEachLoopwithBreak UpdatedActors :!label _label)
      (:LoopBody
        (bind _asmc_char (Utilities|Casting|CastToMC_Char _array_element))
        (if (not (Class|CharPawn|GetIsDead _asmc_char))
          (Variables|Default|SetFindEnemy _asmc_char)
          (Variables|Default|SetFindSomeOne true)
          (goto _label Break)))
      (:Completed
        (if (Variables|Default|GetFindSomeOne)
          (bind _info (Class|AIPerceptionComponent|GetActorsPerception (Variables|Default|GetPerceptionComp) (Variables|Default|GetFindEnemy)))
          (if (.bSuccessfullySensed (Utilities|Struct|BreakAIStimulus (Utilities|Array|Get(acopy) (.LastSensedStimuli (Utilities|Struct|BreakActorPerceptionBlueprintInfo _info)))))
            (AI|Components|Blackboard|SetValueasObject _returnvalue (Utilities|Name|MakeLiteralName "Enemy") (Variables|Default|GetFindEnemy))
            (AI|Components|Blackboard|SetValueasEnum _returnvalue _returnvalue_2 2)
            (Class|AICEnemy|ChangePercepion true (Class|AICEnemy|GetPerceptionLoseRadius) false 0.0 false 0.0)
            (else
              (AI|Components|Blackboard|SetValueasVector _returnvalue (Utilities|Name|MakeLiteralName "Location") (Transformation|GetActorLocation (.Target (Utilities|Struct|BreakActorPerceptionBlueprintInfo _info))))
              (AI|Components|Blackboard|SetValueasEnum _returnvalue _returnvalue_2 1))))))))

(event EventBeginPlay
  (bind _returnvalue (Pawn|GetControlledPawn))
  (bind _returnvalue_2 (AI|GetBlackboard _returnvalue))
  (AI|Components|Blackboard|SetValueasVector _returnvalue_2 (Utilities|Name|MakeLiteralName "DutyLocation") (Transformation|GetActorLocation (Pawn|GetControlledPawn)))
  (AI|Components|Blackboard|SetValueasObject _returnvalue_2 (Utilities|Name|MakeLiteralName "SelfActor") (Pawn|GetControlledPawn)))

(fn ConstructionScript)