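; AI controller for the Tetrohdron enemy that runs its behavior tree and drives facing, dashing and ray-attack state.
; Perception picks a living MC_Char, updates Status and blackboard Enemy or Location, and switches sight to the lose radius once sensed.
; Tick turns the pawn toward Enemy or its velocity, mirrors Status into EnumKey, and after randomized delays dashes to distant Locations.
; RayStart overrides EnumKey and suspends dashing until the ray ends.
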(event OnPerceptionUpdated(PerceptionComp)
  (params (UpdatedActors :type Array%20of%20Actor%20Object%20References))
  (bind _returnvalue (AI|GetBlackboard 0))
  (Variables|Default|SetFindSomeOne false)
  (bind _array_element (Utilities|Array|ForEachLoopwithBreak UpdatedActors :!label _label)
    (:LoopBody
      (bind _asmc_char (Utilities|Casting|CastToMC_Char _array_element))
      (if (not (Class|CharPawn|GetIsDead _asmc_char))
        (Variables|Default|SetFindEnemy _asmc_char)
        (Variables|Default|SetFindSomeOne true)
        (goto _label Break)))
    (:Completed
      (if (Variables|Default|GetFindSomeOne)
        (bind _info (Class|AIPerceptionComponent|GetActorsPerception (Variables|Default|GetPerceptionComp) (Variables|Default|GetFindEnemy)))
        (if (.bSuccessfullySensed (Utilities|Struct|BreakAIStimulus (Utilities|Array|Get(acopy) (.LastSensedStimuli (Utilities|Struct|BreakActorPerceptionBlueprintInfo _info)))))
          (AI|Components|Blackboard|SetValueasObject _returnvalue (Utilities|Name|MakeLiteralName "Enemy") (Variables|Default|GetFindEnemy))
          (Variables|Default|SetStatus "NewEnumerator2")
          (Class|AICEnemy|ChangePercepion true (Class|AICEnemy|GetPerceptionLoseRadius) false 0.0 false 0.0)
          (else
            (AI|Components|Blackboard|SetValueasVector _returnvalue (Utilities|Name|MakeLiteralName "Location") (Transformation|GetActorLocation (.Target (Utilities|Struct|BreakActorPerceptionBlueprintInfo _info))))
            (Variables|Default|SetStatus "NewEnumerator1")))))))

(event Custom|RayStart
  (params (StartEnd :type Boolean))
  (bind _returnvalue (AI|GetBlackboard 0))
  (bind _returnvalue_2 (Utilities|Name|MakeLiteralName "EnumKey"))
  (Variables|Default|SetRayTime StartEnd)
  (if StartEnd
    (AI|Components|Blackboard|SetValueasEnum _returnvalue _returnvalue_2 3)
    (Development|PrintString "Ai Ray started")
    (else
      (AI|Components|Blackboard|SetValueasEnum _returnvalue _returnvalue_2 (Variables|Default|GetStatus))
      (Development|PrintString "AI Ray ended"))))

(event EventBeginPlay
  (AI|RunBehaviorTree "/Game/Game/AI/Tetrohdron/BT_Enemy_Tetrohdron.BT_Enemy_Tetrohdron")
  (Class|LowEntryExtendedStandardLibrary|DelayFrames 1)
  (|CallParentFunction))

(event EventTick
  (params (DeltaSeconds :type Float%20%28single-precision%29))
  (bind _returnvalue (AI|GetBlackboard 0))
  (bind _returnvalue_2 (Utilities|Name|MakeLiteralName "Enemy"))
  (bind _returnvalue_3 (Pawn|GetControlledPawn))
  (bind _returnvalue_4 (AI|GetBlackboard 0))
  (bind _returnvalue_5 (Utilities|Name|MakeLiteralName "Location"))
  (bind _deshdelaydelta (Variables|Default|GetDeshDelayDelta))
  (bind _returnvalue_6 (AI|Components|Blackboard|GetValueasVector _returnvalue_4 _returnvalue_5))
  (bind _returnvalue_7 (AI|Components|Blackboard|GetValueasObject _returnvalue _returnvalue_2))
  (Utilities|FlowControl|Sequence
    (:then_0
      (bind _asenemy_char (Utilities|Casting|CastToEnemy_Char (Pawn|GetControlledPawn)))
      (if true
        (Utilities|IsValid _returnvalue_7
          (:Is%20Valid
            (bind _asactor (Utilities|Casting|CastToActor _returnvalue_7))
            (Class|EnemyChar|InterpFaceArrow _asenemy_char DeltaSeconds (Transformation|GetActorLocation _asactor)))
          (:Is%20Not%20Valid
            (Class|EnemyChar|InterpFaceArrow _asenemy_char DeltaSeconds (+ (Transformation|GetVelocity _asenemy_char) (Transformation|GetActorLocation _asenemy_char)) :!label _label)))
        (else
          (goto _label))))
    (:then_1
      (if (not (Variables|Default|GetRayTime))
        (AI|Components|Blackboard|SetValueasEnum (AI|GetBlackboard 0) (Utilities|Name|MakeLiteralName "EnumKey") (Variables|Default|GetStatus))
        (Utilities|FlowControl|Delay (+ (Math|Random|RandomFloatinRange (* _deshdelaydelta -1.0) _deshdelaydelta) (Variables|Default|GetDeshDelay)))
        (if (not (Variables|Default|GetRayTime))
          (bind _asbp_enemy_wtetrahdron (Utilities|Casting|CastToBP_Enemy_WTetrahdron _returnvalue_3))
          (if (> (Math|Vector|VectorLength (- (Transformation|GetActorLocation _returnvalue_3) _returnvalue_6)) 7e+01)
            (Class|EnemyWTetrahdron|StartDesh _asbp_enemy_wtetrahdron _returnvalue_6)))))))

(event EventSetEnum
  (params (Enum :type E_AIStates%20Enum))
  (Variables|Default|SetStatus Enum))

(fn ConstructionScript
  (|CallParentFunction))