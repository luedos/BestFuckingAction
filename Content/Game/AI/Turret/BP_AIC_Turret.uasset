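; AI controller for an enemy turret that opens, aims and fires at living player characters it perceives.
; Perception updates pick a target, set an enum state, open or close the turret, and switch sight to the lose radius on detection.
; In the engaged state, Tick interpolates yaw toward the target and fires once nearly aligned, with a gate and delay as cooldown.
; It assigns a blackboard but runs no behavior tree.
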(event OnPerceptionUpdated(PerceptionComp)
  (params (UpdatedActors :type Array%20of%20Actor%20Object%20References))
  (Variables|Default|SetFindSomeOne false)
  (bind _array_element (Utilities|Array|ForEachLoopwithBreak UpdatedActors :!label _label)
    (:LoopBody
      (bind _asmc_char (Utilities|Casting|CastToMC_Char _array_element))
      (if (not (Class|CharPawn|GetIsDead _asmc_char))
        (Variables|Default|SetFindEnemy _asmc_char)
        (Variables|Default|SetFindSomeOne true)
        (goto _label Break)))
    (:Completed
      (if (Variables|Default|GetFindSomeOne)
        (bind _info (Class|AIPerceptionComponent|GetActorsPerception (Variables|Default|GetPerceptionComp) (Variables|Default|GetFindEnemy)))
        (if (.bSuccessfullySensed (Utilities|Struct|BreakAIStimulus (Utilities|Array|Get(acopy) (.LastSensedStimuli (Utilities|Struct|BreakActorPerceptionBlueprintInfo _info)))))
          (Variables|Default|SetEnumKey "NewEnumerator2")
          (Class|AICEnemy|ChangePercepion true (Class|AICEnemy|GetPerceptionLoseRadius) false 0.0 false 0.0)
          (bind _asenemy_turret (Utilities|Casting|CastToEnemy_Turret (Pawn|GetControlledPawn)))
          (Class|EnemyTurret|SetOpen _asenemy_turret true)
          (else
            (Variables|Default|SetEnumKey "NewEnumerator3")
            (bind _asenemy_turret_2 (Utilities|Casting|CastToEnemy_Turret (Pawn|GetControlledPawn)))
            (Class|EnemyTurret|SetOpen _asenemy_turret_2 false)))))))

(event EventTick
  (params (DeltaSeconds :type Float%20%28single-precision%29))
  (bind _returnvalue (Pawn|GetControlledPawn))
  (bind _returnvalue_2 (Pawn|GetControlledPawn))
  (bind _findenemy (Variables|Default|GetFindEnemy))
  (bind _enumkey (Variables|Default|GetEnumKey))
  (bind _returnvalue_3 (Transformation|GetActorLocation _returnvalue))
  (bind _returnvalue_4 (Transformation|GetActorLocation _findenemy))
  (bind _returnvalue_5 (Transformation|GetActorRotation _returnvalue_2))
  (bind _returnvalue_6 (Math|Rotator|FindLookatRotation _returnvalue_3 _returnvalue_4))
  (bind _yaw (Math|Rotator|BreakRotator _returnvalue_6))
  (bind _asbp_enemy_turret (Utilities|Casting|CastToBP_Enemy_Turret (Pawn|GetControlledPawn)))
  (if (and (Utilities|Enum|Equal(Enum) _enumkey "NewEnumerator0") (Variables|/Game/Game/Character/BP_Enemy_Turret.BP_Enemy_Turret_C|GetIsOpen _asbp_enemy_turret))
    (Class|EnemyTurret|SetOpen _asbp_enemy_turret false)
    (elif (Utilities|Enum|Equal(Enum) _enumkey "NewEnumerator2")
      (Transformation|SetActorRotation _returnvalue_2 (Math|Interpolation|RInterpTo (Math|Rotator|MakeRotator 0.0 0.0 (.yaw _returnvalue_5)) (Math|Rotator|MakeRotator 0.0 0.0 _yaw) DeltaSeconds 1e+01))
      (if (Math|Float|NearlyEqual(Float) (.yaw _returnvalue_5) _yaw 15.0)
        (Utilities|FlowControl|Gate false :!label _label
          (:Exit
            (bind _asenemy_char (Utilities|Casting|CastToEnemy_Char (Pawn|GetControlledPawn)))
            (Class|EnemyChar|EnemyFire _asenemy_char 1 0 false)
            (Utilities|FlowControl|Sequence
              (:then_0
                (goto _label Close))
              (:then_1
                (Utilities|FlowControl|Delay 2.0)
                (goto _label Open)))))))))

(event EventBeginPlay
  (Class|AIController|UseBlackboard "/Game/Game/AI/Tetrohdron/BB_Enemy_WTetrohdron.BB_Enemy_WTetrohdron"))

(event EventSetEnum
  (params (Enum :type E_AIStates%20Enum))
  (Variables|Default|SetEnumKey Enum))

(fn ConstructionScript)